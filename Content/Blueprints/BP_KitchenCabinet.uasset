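; Kitchen cabinet Blueprint with two hinged doors that each toggle open and closed independently through the OpenClose event.
; The component passed in selects the door, and a shared Locked flag plays a locked sound instead of moving it.
; Each door has an open flag and opposing timed MoveComponentTo nodes, with the reverse move stopped on each toggle.
; Open and close sound nodes and an older instant-move branch are left unconnected.
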(event EventBeginPlay)

(event EventOpenClose
  (params (Component :type Primitive%20Component%20Object%20Reference))
  (bind _door1 (Variables|Default|GetDoor1))
  (bind _door (Variables|Default|GetDoor))
  (if (== Component (Variables|Default|GetDoor))
    (if (Variables|Default|GetLocked)
      (Audio|PlaySoundatLocation "/Game/Sounds/LockedDoor_Cue.LockedDoor_Cue" (Transformation|GetActorLocation) "0, 0, 0" 1.0 1.0 0.0 "/Game/Sounds/Attenuation/DoorSoundAttenuation.DoorSoundAttenuation" 0 0 :!label _label)
      (elif (Variables|Default|GetOpen)
        (Utilities|FlowControl|Sequence
          (:then_0
            (Variables|Default|SetOpen false)
            (Components|MoveComponentTo _door "32.000000,14.000000,3.000000" "0, 0, 0" false false 0.5 false :!label _label_2))
          (:then_1
            (goto _label_3 Stop)))
        (else
          (Utilities|FlowControl|Sequence
            (:then_0
              (Variables|Default|SetOpen true)
              (Components|MoveComponentTo _door "32.000000,14.000000,3.000000" "0,-95.000000, 0" false false 0.5 false :!label _label_3))
            (:then_1
              (goto _label_2 Stop))))))
    (elif (== Component (Variables|Default|GetDoor1))
      (if (Variables|Default|GetLocked)
        (goto _label)
        (elif (Variables|Default|GetOpen_1)
          (Utilities|FlowControl|Sequence
            (:then_0
              (Variables|Default|SetOpen_1 false)
              (Components|MoveComponentTo _door1 "-31.600000,14.000000,3.000000" "0, 0, 0" false false 0.5 false :!label _label_4))
            (:then_1
              (goto _label_5 Stop)))
          (else
            (Utilities|FlowControl|Sequence
              (:then_0
                (Variables|Default|SetOpen_1 true)
                (Components|MoveComponentTo _door1 "-31.600000,14.000000,3.000000" "0,95.000000, 0" false false 0.5 false :!label _label_5))
              (:then_1
                (goto _label_4 Stop)))))))))

(fn ConstructionScript
  (|CallParentFunction))