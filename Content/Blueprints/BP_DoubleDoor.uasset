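; Double door actor whose two leaves open and close independently, or play a locked sound.
; OpenClose toggles the given leaf with timed component moves, stopping the opposite move and switching collision to physics-only during motion.
; When CanAIOpen is set, a smart nav link swings Door1 for AI, pausing their movement, or waiting longer if chair-blocked, then closes it.
; An older BP_Neighbor opening sequence remains unconnected.
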(event OnSmartLinkReached(NavLink)
  (params (MovingActor :type Actor%20Object%20Reference) (DestinationPoint :type Vector%20%28by%20ref%29 :default "0, 0, 0"))
  (bind _door1 (Variables|Default|GetDoor1))
  (bind _door1_2 (Variables|Default|GetDoor1))
  (bind _asai (Utilities|Casting|CastToAI MovingActor))
  (if (Variables|Default|GetCanAIOpen?)
    (if (Variables|Default|GetIsLockedWithChair?)
      (Utilities|FlowControl|Delay 4.2)
      (Components|MoveComponentTo (Variables|Default|GetDoor1) "170.000000,10.000000, 0" "0,-280.000000, 0" false false 0.1 false)
      (elif (Variables|Default|GetOpen_1)
        (Utilities|FlowControl|Delay 1.24)
        (else
          (Pawn|Components|CharacterMovement|DisableMovement (Variables|/Script/Engine.Character|GetCharacterMovement _asai))
          (Components|Animation|SetAnimationMode (Variables|/Script/Engine.Character|GetMesh _asai) "AnimationSingleNode")
          (Utilities|FlowControl|Delay 0.4)
          (Variables|Default|SetOpen_1 true)
          (Components|MoveComponentTo _door1 "170.000000,10.000000, 0" "0,-280.000000,0.000000" false false 0.5 false)
          (Collision|SetCollisionEnabled _door1 "PhysicsOnly")
          (Utilities|FlowControl|Delay 0.54)
          (Components|Animation|SetAnimationMode (Variables|/Script/Engine.Character|GetMesh _asai) "AnimationBlueprint")
          (Pawn|Components|CharacterMovement|SetMovementMode (Variables|/Script/Engine.Character|GetCharacterMovement _asai) "MOVE_Walking" 0))))
    (Utilities|FlowControl|Delay 1.5)
    (Components|MoveComponentTo _door1_2 "170.000000,10.000000,0.000000" "0,-180.000000, 0" false false 0.5 false)
    (Collision|SetCollisionEnabled _door1_2 "QueryAndPhysics")
    (Variables|Default|SetOpen_1 false)))

(event EventBeginPlay
  (bind _door1 (Variables|Default|GetDoor1))
  (if (Variables|Default|GetOpen_1)
    (Transformation|SetRelativeLocationAndRotation _door1 "170.000000,10.000000, 0" "0,-280.000000, 0" false false)
    (else
      (Transformation|SetRelativeLocationAndRotation _door1 "170.000000,10.000000, 0" (Variables|Default|GetNew%20Rotation) false false))))

(event EventOpenClose
  (params (Component :type Primitive%20Component%20Object%20Reference))
  (bind _door1 (Variables|Default|GetDoor1))
  (bind _door (Variables|Default|GetDoor))
  (if (== Component (Variables|Default|GetDoor))
    (if (Variables|Default|GetLocked)
      (Audio|PlaySoundatLocation "/Game/Sounds/LockedDoor_Cue.LockedDoor_Cue" (Transformation|GetWorldLocation (Variables|Default|GetScene)) "0, 0, 0" 1.0 1.0 0.0 "/Game/Sounds/Attenuation/DoorSoundAttenuation.DoorSoundAttenuation" 0 0 :!label _label)
      (elif (Variables|Default|GetOpen)
        (Utilities|FlowControl|Sequence
          (:then_0
            (Collision|SetCollisionEnabled _door "PhysicsOnly")
            (Components|MoveComponentTo _door "-1.000000,10.000000, 0" "0, 0, 0" false false 0.5 false :!label _label_2)
            (Audio|SpawnSoundatLocation (Variables|Default|GetCloseSound) (Transformation|GetWorldLocation (Variables|Default|GetScene)) "0, 0, 0" 1.0 1.0 0.0 "/Game/Sounds/Attenuation/DoorSoundAttenuation.DoorSoundAttenuation" 0)
            (Collision|SetCollisionEnabled _door "QueryAndPhysics")
            (Variables|Default|SetOpen false))
          (:then_1
            (goto _label_3 Stop)))
        (else
          (Utilities|FlowControl|Sequence
            (:then_0
              (Variables|Default|SetOpen true)
              (Collision|SetCollisionEnabled _door "PhysicsOnly")
              (Components|MoveComponentTo _door "-1.000000,10.000000, 0" "0,100.000000, 0" false false 0.5 false :!label _label_3)
              (Collision|SetCollisionEnabled _door "QueryAndPhysics"))
            (:then_1
              (goto _label_2 Stop))
            (:then_2
              (Audio|SpawnSoundatLocation "/Game/Sounds/Entrance_Door_Open.Entrance_Door_Open" (Transformation|GetWorldLocation (Variables|Default|GetScene)) "0, 0, 0" 1.0 1.0 0.0 "/Game/Sounds/Attenuation/DoorSoundAttenuation.DoorSoundAttenuation" 0))))))
    (elif (== Component (Variables|Default|GetDoor1))
      (if (Variables|Default|GetLocked)
        (goto _label)
        (elif (Variables|Default|GetOpen_1)
          (Utilities|FlowControl|Sequence
            (:then_0
              (Collision|SetCollisionEnabled _door1 "PhysicsOnly")
              (Components|MoveComponentTo _door1 "170.000000,10.000000, 0" "0,-180.000000, 0" false false 0.5 false :!label _label_4)
              (Audio|SpawnSoundatLocation (Variables|Default|GetCloseSound) (Transformation|GetWorldLocation (Variables|Default|GetScene)) "0, 0, 0" 1.0 1.0 0.0 "/Game/Sounds/Attenuation/DoorSoundAttenuation.DoorSoundAttenuation" 0)
              (Collision|SetCollisionEnabled _door1 "QueryAndPhysics")
              (Variables|Default|SetOpen_1 false))
            (:then_1
              (goto _label_5 Stop)))
          (else
            (Utilities|FlowControl|Sequence
              (:then_0
                (Variables|Default|SetOpen_1 true)
                (Collision|SetCollisionEnabled _door1 "PhysicsOnly")
                (Components|MoveComponentTo _door1 "170.000000,10.000000, 0" "0,-280.000000, 0" false false 0.5 false :!label _label_5)
                (Collision|SetCollisionEnabled _door1 "QueryAndPhysics"))
              (:then_1
                (goto _label_4 Stop))
              (:then_2
                (Audio|SpawnSoundatLocation "/Game/Sounds/Entrance_Door_Open.Entrance_Door_Open" (Transformation|GetWorldLocation (Variables|Default|GetScene)) "0, 0, 0" 1.0 1.0 0.0 "/Game/Sounds/Attenuation/DoorSoundAttenuation.DoorSoundAttenuation" 0)))))))))

(fn ConstructionScript
  (|CallParentFunction))