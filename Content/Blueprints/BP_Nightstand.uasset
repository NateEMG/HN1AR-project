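; Nightstand Blueprint with two sliding drawers, Door and Door1, that toggle open and closed with sound.
; OpenClose matches the passed component to a drawer, playing a locked sound if Locked is set, otherwise flipping that drawer's open flag.
; Each drawer uses paired MoveComponentTo nodes, stopping the opposite move when one starts.
; BeginPlay snaps only Door1 to its initial position from Open1.
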(event EventBeginPlay
  (bind _door1 (Variables|Default|GetDoor1))
  (if (Variables|Default|GetOpen_1)
    (Transformation|SetRelativeLocationAndRotation _door1 "0.000000,40.000000,18.000000" "0, 0, 0" false false)
    (else
      (Transformation|SetRelativeLocationAndRotation _door1 "0.000000,-1.000000,18.000000" "0, 0, 0" false false))))

(event EventOpenClose
  (params (Component :type Primitive%20Component%20Object%20Reference))
  (bind _door1 (Variables|Default|GetDoor1))
  (bind _door (Variables|Default|GetDoor))
  (if (== Component (Variables|Default|GetDoor))
    (if (Variables|Default|GetLocked)
      (Audio|PlaySoundatLocation "/Game/Sounds/LockedDoor_Cue.LockedDoor_Cue" (Transformation|GetActorLocation) "0, 0, 0" 1.0 1.0 0.0 "/Game/Sounds/Attenuation/DoorSoundAttenuation.DoorSoundAttenuation" 0 0 :!label _label)
      (elif (Variables|Default|GetOpen)
        (Utilities|FlowControl|Sequence
          (:then_0
            (Variables|Default|SetOpen false)
            (Components|MoveComponentTo _door "0,-1.000000,0.000000" "0, 0, 0" false false 0.6 false :!label _label_2))
          (:then_1
            (goto _label_3 Stop))
          (:then_2
            (Audio|SpawnSoundatLocation "/Game/Sounds/drawer_close_Cue.drawer_close_Cue" (Transformation|GetActorLocation) "0, 0, 0" 1.0 1.0 0.0 "/Game/Sounds/Attenuation/ItemAtten.ItemAtten" 0)))
        (else
          (Utilities|FlowControl|Sequence
            (:then_0
              (Variables|Default|SetOpen true)
              (Components|MoveComponentTo _door "0,40.000000,0.000000" "0, 0, 0" false false 0.5 false :!label _label_3))
            (:then_1
              (goto _label_2 Stop))
            (:then_2
              (Audio|SpawnSoundatLocation "/Game/Sounds/drawer_open_Cue.drawer_open_Cue" (Transformation|GetActorLocation) "0, 0, 0" 1.0 1.0 0.0 "/Game/Sounds/Attenuation/ItemAtten.ItemAtten" 0))))))
    (elif (== Component (Variables|Default|GetDoor1))
      (if (Variables|Default|GetLocked)
        (goto _label)
        (elif (Variables|Default|GetOpen_1)
          (Utilities|FlowControl|Sequence
            (:then_0
              (Variables|Default|SetOpen_1 false)
              (Components|MoveComponentTo _door1 "0.000000,-1.000000,18.000000" "0, 0, 0" false false 0.6 false :!label _label_4))
            (:then_1
              (goto _label_5 Stop))
            (:then_2
              (Audio|SpawnSoundatLocation "/Game/Sounds/drawer_close_Cue.drawer_close_Cue" (Transformation|GetActorLocation) "0, 0, 0" 1.0 1.0 0.0 "/Game/Sounds/Attenuation/ItemAtten.ItemAtten" 0)))
          (else
            (Utilities|FlowControl|Sequence
              (:then_0
                (Variables|Default|SetOpen_1 true)
                (Components|MoveComponentTo _door1 "0.000000,40.000000,18.000000" "0, 0, 0" false false 0.5 false :!label _label_5))
              (:then_1
                (goto _label_4 Stop))
              (:then_2
                (Audio|SpawnSoundatLocation "/Game/Sounds/drawer_open_Cue.drawer_open_Cue" (Transformation|GetActorLocation) "0, 0, 0" 1.0 1.0 0.0 "/Game/Sounds/Attenuation/ItemAtten.ItemAtten" 0))))))
      (elif (== Component 0)
        (if true
          _)))))

(fn ConstructionScript
  (|CallParentFunction))