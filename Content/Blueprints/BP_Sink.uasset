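; BP_Sink is a sink actor with four doors that open and close individually.
; OpenClose matches the passed component to a door, flips its open flag and moves it to a stored open or closed transform over half a second, stopping the opposing move.
; A shared Locked flag makes the first two doors play a locked sound instead of moving.
; Open and close sound nodes exist but are disconnected.
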(event EventBeginPlay)

(event EventOpenClose
  (params (Component :type Primitive%20Component%20Object%20Reference))
  (bind _door_3_open (Variables|Default|GetDoor%203%20Open))
  (bind _door_3_close (Variables|Default|GetDoor%203%20Close))
  (bind _door_2_open_transform (Variables|Default|GetDoor%202%20Open%20Transform))
  (bind _door2 (Variables|Default|GetDoor2))
  (bind _door3 (Variables|Default|GetDoor3))
  (bind _door_2_close_transform (Variables|Default|GetDoor%202%20Close%20Transform))
  (bind _door_1_open_transform (Variables|Default|GetDoor%201%20Open%20Transform))
  (bind _door_1_close_transform (Variables|Default|GetDoor%201%20Close%20Transform))
  (bind _door_4_open (Variables|Default|GetDoor%204%20Open))
  (bind _door_4_close (Variables|Default|GetDoor%204%20Close))
  (bind _door (Variables|Default|GetDoor))
  (bind _door1 (Variables|Default|GetDoor1))
  (if (== Component (Variables|Default|GetDoor))
    (if (Variables|Default|GetLocked)
      (Audio|PlaySoundatLocation "/Game/Sounds/LockedDoor_Cue.LockedDoor_Cue" (Transformation|GetActorLocation) "0, 0, 0" 1.0 1.0 0.0 "/Game/Sounds/Attenuation/DoorSoundAttenuation.DoorSoundAttenuation" 0 0 :!label _label)
      (elif (Variables|Default|GetOpen)
        (Utilities|FlowControl|Sequence
          (:then_0
            (Variables|Default|SetOpen false)
            (Components|MoveComponentTo _door (.location _door_1_close_transform) (.rotation _door_1_close_transform) false false 0.5 false :!label _label_2))
          (:then_1
            (goto _label_3 Stop)))
        (else
          (Utilities|FlowControl|Sequence
            (:then_0
              (Variables|Default|SetOpen true)
              (Components|MoveComponentTo _door (.location _door_1_open_transform) (.rotation _door_1_open_transform) false false 0.5 false :!label _label_3))
            (:then_1
              (goto _label_2 Stop))))))
    (elif (== Component (Variables|Default|GetDoor1))
      (if (Variables|Default|GetLocked)
        (goto _label)
        (elif (Variables|Default|GetOpen_1)
          (Utilities|FlowControl|Sequence
            (:then_0
              (Variables|Default|SetOpen_1 false)
              (Components|MoveComponentTo _door1 (.location _door_2_close_transform) (.rotation _door_2_close_transform) false false 0.5 false :!label _label_4))
            (:then_1
              (goto _label_5 Stop)))
          (else
            (Utilities|FlowControl|Sequence
              (:then_0
                (Variables|Default|SetOpen_1 true)
                (Components|MoveComponentTo _door1 (.location _door_2_open_transform) (.rotation _door_2_open_transform) false false 0.5 false :!label _label_5))
              (:then_1
                (goto _label_4 Stop))))))
      (elif (== Component (Variables|Default|GetDoor2))
        (if (Variables|Default|GetOpen_2)
          (Utilities|FlowControl|Sequence
            (:then_0
              (Variables|Default|SetOpen_2 false)
              (Components|MoveComponentTo _door2 (.location _door_3_close) (.rotation _door_3_close) false false 0.5 false :!label _label_6))
            (:then_1
              (goto _label_7 Stop)))
          (else
            (Utilities|FlowControl|Sequence
              (:then_0
                (Variables|Default|SetOpen_2 true)
                (Components|MoveComponentTo _door2 (.location _door_3_open) (.rotation _door_3_open) false false 0.5 false :!label _label_7))
              (:then_1
                (goto _label_6 Stop)))))
        (elif (== Component (Variables|Default|GetDoor3))
          (if (Variables|Default|Getopen3)
            (Utilities|FlowControl|Sequence
              (:then_0
                (Variables|Default|Setopen3 false)
                (Components|MoveComponentTo _door3 (.location _door_4_close) (.rotation _door_4_close) false false 0.5 false :!label _label_8))
              (:then_1
                (goto _label_9 Stop)))
            (else
              (Utilities|FlowControl|Sequence
                (:then_0
                  (Variables|Default|Setopen3 true)
                  (Components|MoveComponentTo _door3 (.location _door_4_open) (.rotation _door_4_open) false false 0.5 false :!label _label_9))
                (:then_1
                  (goto _label_8 Stop))))))))))

(fn ConstructionScript
  (|CallParentFunction))