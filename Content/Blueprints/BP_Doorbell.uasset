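; BP_Doorbell is an interactable doorbell that plays a chime and lures the AI toward it.
; On Interact it plays a spatialized ding-dong sound and reports a tagged noise event at a linked bell point for AI hearing.
; It also writes itself into the first found AI's blackboard as ObjectRef.
; A DoOnce reset after a short delay prevents repeated ringing.
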(event Custom|Interact
  (bind _self self)
  (Utilities|FlowControl|DoOnce false :!label _label
    (:Completed
      (Audio|PlaySoundatLocation "/Game/Sounds/ding_dong_Cue.ding_dong_Cue" (Transformation|GetActorLocation) "0, 0, 0" 1.0 1.0 0.0 "/Game/Sounds/Attenuation/DoorSoundAttenuation.DoorSoundAttenuation" 0 0)
      (Class|AISenseHearing|ReportNoiseEvent (Transformation|GetActorLocation (Variables|Default|GetDoorBellPoint)) 5.0 _self 1.2e+03 "Doorbell")
      (bind _returnvalue (Actor|GetActorOfClass "/Game/Blueprints/Characters/AI2/AI.AI_C"))
      (AI|Components|Blackboard|SetValueasObject (AI|GetBlackboard _returnvalue) (Utilities|Name|MakeLiteralName "ObjectRef") _self)
      (Utilities|FlowControl|Delay 1.5)
      (goto _label Reset))))

(event EventBeginPlay)

(event Collision|EventActorBeginOverlap
  (params (OtherActor :type Actor%20Object%20Reference)))

(event EventTick
  (params (DeltaSeconds :type Float%20%28single-precision%29)))

(fn ConstructionScript)