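; Kitchen counter actor with three cabinet doors that swing open and closed individually.
; OpenClose receives the targeted component, toggles that door's open flag and animates it with paired MoveComponentTo nodes, stopping the opposite move so it can reverse mid-swing.
; A shared Locked flag blocks all three doors and plays a locked-door sound instead.
; Open and close sound nodes and an older snap-move of Door1 are left unwired.
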(event EventBeginPlay)

(event EventOpenClose
  (params (Component :type Primitive%20Component%20Object%20Reference))
  (bind _door1 (Variables|Default|GetDoor1))
  (bind _door2 (Variables|Default|GetDoor2))
  (bind _door (Variables|Default|GetDoor))
  (if (== Component (Variables|Default|GetDoor))
    (if (Variables|Default|GetLocked)
      (Audio|PlaySoundatLocation "/Game/Sounds/LockedDoor_Cue.LockedDoor_Cue" (Transformation|GetActorLocation) "0, 0, 0" 1.0 1.0 0.0 "/Game/Sounds/Attenuation/DoorSoundAttenuation.DoorSoundAttenuation" 0 0 :!label _label)
      (elif (Variables|Default|GetOpen)
        (Utilities|FlowControl|Sequence
          (:then_0
            (Variables|Default|SetOpen false)
            (Components|MoveComponentTo _door "14.000000,25.000000,13.000000" "0, 0, 0" false false 0.5 false :!label _label_2))
          (:then_1
            (goto _label_3 Stop)))
        (else
          (Utilities|FlowControl|Sequence
            (:then_0
              (Variables|Default|SetOpen true)
              (Components|MoveComponentTo _door "14.000000,25.000000,13.000000" "0,-95.000000, 0" false false 0.5 false :!label _label_3))
            (:then_1
              (goto _label_2 Stop))))))
    (elif (== Component (Variables|Default|GetDoor1))
      (if (Variables|Default|GetLocked)
        (goto _label)
        (elif (Variables|Default|GetOpen_1)
          (Utilities|FlowControl|Sequence
            (:then_0
              (Variables|Default|SetOpen_1 false)
              (Components|MoveComponentTo _door1 "-54.000000,25.000000,13.000000" "0, 0, 0" false false 0.5 false :!label _label_4))
            (:then_1
              (goto _label_5 Stop)))
          (else
            (Utilities|FlowControl|Sequence
              (:then_0
                (Variables|Default|SetOpen_1 true)
                (Components|MoveComponentTo _door1 "-54.000000,25.000000,13.000000" "0,95.000000, 0" false false 0.5 false :!label _label_5))
              (:then_1
                (goto _label_4 Stop))))))
      (elif (== Component (Variables|Default|GetDoor2))
        (if (Variables|Default|GetLocked)
          (goto _label)
          (elif (Variables|Default|GetOpen_2)
            (Utilities|FlowControl|Sequence
              (:then_0
                (Variables|Default|SetOpen_2 false)
                (Components|MoveComponentTo _door2 "53.000000,25.000000,13.000000" "0, 0, 0" false false 0.5 false :!label _label_6))
              (:then_1
                (goto _label_7 Stop)))
            (else
              (Utilities|FlowControl|Sequence
                (:then_0
                  (Variables|Default|SetOpen_2 true)
                  (Components|MoveComponentTo _door2 "53.000000,25.000000,13.000000" "0,-95.000000, 0" false false 0.5 false :!label _label_7))
                (:then_1
                  (goto _label_6 Stop))))))))))

(fn ConstructionScript
  (|CallParentFunction))