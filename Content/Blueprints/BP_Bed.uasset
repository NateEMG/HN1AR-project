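; Bed actor whose Sleep event plays the WakeUp sequence, briefly locks player input and moves the player to the bed point.
; After a delay, it steps the sky through four time-of-day presets by exact float matching, except in level Alpha2, and triggers a weather change, sometimes random.
; In parallel, an awake AI returns to spawn, pauses, drops any held item at its start transform, forgets perception and picks a random task.
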(event Custom|Sleep
  (bind _returnvalue (Game|GetPlayerController 0))
  (bind _bedpointplayer (Variables|Default|GetBedPointPlayer))
  (bind _weatherbp (Variables|Default|GetWeatherBP))
  (bind _skybp (Variables|Default|GetSkyBP))
  (bind _ai (Variables|Default|GetAI))
  (bind _arrow (Variables|/Game/Blueprints/CharacterPoints/BedPointPlayer.BedPointPlayer_C|GetArrow _bedpointplayer))
  (bind _spawntransform (Variables|/Game/Blueprints/Characters/AI2/AI.AI_C|GetSpawnTransform _ai))
  (bind _charactermovement (Variables|/Script/Engine.Character|GetCharacterMovement _ai))
  (bind _currentitem (Variables|/Game/Blueprints/Characters/AI2/AI.AI_C|GetCurrentItem _ai))
  (bind _returnvalue_2 (Sequencer|Player|CreateLevelSequencePlayer "/Game/Blueprints/LevelSequences/WakeUp.WakeUp"))
  (Sequencer|Player|Play _returnvalue_2 :!class /Script/MovieScene.MovieSceneSequencePlayer)
  (bind _asfirst_person_character (Utilities|Casting|CastToFirstPersonCharacter (Game|GetPlayerCharacter 0)))
  (Input|DisableInput _asfirst_person_character _returnvalue)
  (Utilities|FlowControl|Sequence
    (:then_0
      (Utilities|FlowControl|Delay 2.34)
      (Utilities|FlowControl|Sequence
        (:then_0
          (Utilities|FlowControl|Delay 1.39)
          (Input|EnableInput _asfirst_person_character _returnvalue))
        (:then_1
          (Transformation|SetActorLocationAndRotation _asfirst_person_character (Transformation|GetWorldLocation _arrow) (Transformation|GetWorldRotation _arrow)))
        (:then_2
          (bind _returnvalue_3 (Game|GetCurrentLevelName true))
          (if (not (Utilities|Enum|Equal(Enum) _returnvalue_3 "Alpha2"))
            (if (== (Variables|/Game/UltraDynamicSky/Blueprints/Ultra_Dynamic_Sky.Ultra_Dynamic_Sky_C|GetTime%20of%20Day _skybp) 665.714172)
              (Variables|/Game/UltraDynamicSky/Blueprints/Ultra_Dynamic_Sky.Ultra_Dynamic_Sky_C|SetTime%20of%20Day _skybp 8e+02)
              (Variables|/Game/UltraDynamicSky/Blueprints/Ultra_Dynamic_Sky.Ultra_Dynamic_Sky_C|SetSky%20Light%20Intensity _skybp 0.2 :!label _label)
              (elif (== (Variables|/Game/UltraDynamicSky/Blueprints/Ultra_Dynamic_Sky.Ultra_Dynamic_Sky_C|GetTime%20of%20Day _skybp) 8e+02)
                (Variables|/Game/UltraDynamicSky/Blueprints/Ultra_Dynamic_Sky.Ultra_Dynamic_Sky_C|SetTime%20of%20Day _skybp 1691.428711)
                (goto _label)
                (elif (== (Variables|/Game/UltraDynamicSky/Blueprints/Ultra_Dynamic_Sky.Ultra_Dynamic_Sky_C|GetTime%20of%20Day _skybp) 1691.428711)
                  (Variables|/Game/UltraDynamicSky/Blueprints/Ultra_Dynamic_Sky.Ultra_Dynamic_Sky_C|SetTime%20of%20Day _skybp 1965.714478)
                  (Variables|/Game/UltraDynamicSky/Blueprints/Ultra_Dynamic_Sky.Ultra_Dynamic_Sky_C|SetSky%20Light%20Intensity _skybp 1.0)
                  (elif (== (Variables|/Game/UltraDynamicSky/Blueprints/Ultra_Dynamic_Sky.Ultra_Dynamic_Sky_C|GetTime%20of%20Day _skybp) 1965.714478)
                    (Variables|/Game/UltraDynamicSky/Blueprints/Ultra_Dynamic_Sky.Ultra_Dynamic_Sky_C|SetTime%20of%20Day _skybp 665.714172)
                    (goto _label)))))))
        (:then_3
          (if (== (Math|Random|RandomIntegerinRange 0 1) 1)
            (Default|ChangeWeatherUsingType _weatherbp (Utilities|Enum|ByteToEnumUDS_WeatherTypes (Math|Conversions|ToByte(Integer) (Math|Random|RandomIntegerinRange 0 7))) 0.5 9e+01 1.2e+02 false)
            (else
              (Default|ChangeWeatherUsingType _weatherbp "NewEnumerator1" 0.5 9e+01 1.2e+02 false))))))
    (:then_1
      (if (not (Variables|/Game/Blueprints/Characters/AI2/AI.AI_C|GetIsSleeping _ai))
        (Transformation|SetActorLocationAndRotation _ai (.location _spawntransform) (.rotation _spawntransform))
        (Default|SetState _ai "NewEnumerator7")
        (Pawn|Components|CharacterMovement|DisableMovement _charactermovement)
        (Utilities|FlowControl|Delay 3.0)
        (Utilities|IsValid _currentitem
          (:Is%20Valid
            (Default|DropItem _ai _currentitem (Variables|/Game/Blueprints/PickUpObjects/BP_Interactable.BP_Interactable_C|GetStartTransform _currentitem)))
          (:Is%20Not%20Valid
            _))
        (Default|SetState _ai "NewEnumerator0")
        (Default|RandomTask _ai)
        (Variables|/Game/Blueprints/Characters/AI2/AI.AI_C|SetCanSeePlayer _ai false)
        (Class|AIPerceptionComponent|ForgetAll (Variables|/Game/Blueprints/Characters/AI2/AI.AI_C|GetAIPerception _ai))
        (Pawn|Components|CharacterMovement|SetMovementMode _charactermovement "MOVE_Walking" 0)))))

(event EventBeginPlay)

(event Collision|EventActorBeginOverlap
  (params (OtherActor :type Actor%20Object%20Reference)))

(event EventTick
  (params (DeltaSeconds :type Float%20%28single-precision%29)))

(fn ConstructionScript)