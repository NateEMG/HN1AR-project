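; BP_Key_player is the key the player holds, used to unlock a BP_Lock with a matching code.
; SetSocket stores the first-person character's Key component as its socket.
; Use traces from the character and, if the lock matches and is not yet pickable, disables input and swaps the key mesh for the lock's animated one.
; After a timed delay it unlocks and detaches the door reference, makes the lock pickable and restores input.
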(event EventBeginPlay
  (|CallParentFunction) ; This node is disabled and will not be called.\nDrag off pins to build functionality.
)

(event Collision|EventActorBeginOverlap
  (params (OtherActor :type Actor%20Object%20Reference)))

(event EventTick
  (params (DeltaSeconds :type Float%20%28single-precision%29)))

(event EventSetSocket
  (bind _asfirst_person_character (Utilities|Casting|CastToFirstPersonCharacter (Game|GetPlayerCharacter 0)))
  (Variables|Default|SetSocket (Variables|/Game/Blueprints/Characters/FirstPersonBP/Blueprints/FirstPersonCharacter.FirstPersonCharacter_C|GetKey _asfirst_person_character)))

(event EventUse
  (bind _returnvalue (Game|GetPlayerController 0))
  (bind _staticmesh (Variables|Default|GetStaticMesh))
  (bind _asfirst_person_character (Utilities|Casting|CastToFirstPersonCharacter (Game|GetPlayerCharacter 0)))
  (bind (_out_hit _return_value) (Default|Trace _asfirst_person_character "TraceTypeQuery1"))
  (if _return_value
    (bind _asbp_lock (Utilities|Casting|CastToBP_Lock (.HitActor (Collision|BreakHitResult _out_hit))))
    (if (Utilities|Enum|Equal(Enum) (Variables|/Game/Blueprints/PickUpObjects/BP_Lock.BP_Lock_C|GetCode _asbp_lock) (Variables|Default|GetCode))
      (if (not (Variables|/Game/Blueprints/PickUpObjects/BP_Interactable.BP_Interactable_C|GetCanPickUp? _asbp_lock))
        (Input|DisableInput _asfirst_person_character _returnvalue)
        (Rendering|SetVisibility _staticmesh false false)
        (Components|Animation|PlayAnimation (Variables|/Game/Blueprints/PickUpObjects/BP_Lock.BP_Lock_C|GetSkeletalMesh _asbp_lock) "/Game/Objects/Meshes/Animated/key/keyplayer.keyplayer" false)
        (Rendering|SetVisibility (Variables|/Game/Blueprints/PickUpObjects/BP_Lock.BP_Lock_C|GetSkeletalMesh _asbp_lock) true false)
        (Utilities|FlowControl|Delay 1.957)
        (Variables|/Game/Blueprints/BP_Door.BP_Door_C|SetLocked (Variables|/Game/Blueprints/PickUpObjects/BP_Lock.BP_Lock_C|GetDoor _asbp_lock) false)
        (Variables|/Game/Blueprints/PickUpObjects/BP_Interactable.BP_Interactable_C|SetCanPickUp? _asbp_lock true)
        (Variables|/Game/Blueprints/PickUpObjects/BP_Lock.BP_Lock_C|SetDoor _asbp_lock 0)
        (Rendering|SetVisibility _staticmesh true false)
        (Rendering|SetVisibility (Variables|/Game/Blueprints/PickUpObjects/BP_Lock.BP_Lock_C|GetSkeletalMesh _asbp_lock) false false)
        (Input|EnableInput _asfirst_person_character _returnvalue)))))

(fn ConstructionScript
  (|CallParentFunction))