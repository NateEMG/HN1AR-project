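; BP_Lock is a pickup-object lock that keeps its assigned door locked, with its nav smart link disabled, until unlocked.
; Tick treats the mesh starting to simulate physics as the unlock, freeing the door and link and playing a creak.
; Its Code string selects which unlock flag to set in the game instance's save data before saving puzzle progress.
; SetSocket assigns the player character's Lock component as its socket.
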(event EventBeginPlay
  (bind _door (Variables|Default|GetDoor))
  (bind _navlink (Variables|/Game/Blueprints/BP_Door.BP_Door_C|GetNavLink _door))
  (|CallParentFunction)
  (Utilities|IsValid _door
    (:Is%20Valid
      (Variables|/Game/Blueprints/BP_Door.BP_Door_C|SetLocked _door true)
      (Variables|Default|SetCanPickUp? false)
      (Variables|Default|SetUnlocked? false)
      (Utilities|IsValid _navlink
        (:Is%20Valid
          (Class|NavLinkProxy|SetSmartLinkEnabled _navlink false))))))

(event Collision|EventActorBeginOverlap
  (params (OtherActor :type Actor%20Object%20Reference)))

(event EventTick
  (params (DeltaSeconds :type Float%20%28single-precision%29))
  (bind _code (Variables|Default|GetCode))
  (Utilities|IsValid (Variables|Default|GetDoor)
    (:Is%20Valid
      (if (Physics|IsSimulatingPhysics (Variables|Default|GetStaticMesh) "None")
        (Utilities|FlowControl|DoOnce false :!label _label
          (:Completed
            (Variables|/Game/Blueprints/BP_Door.BP_Door_C|SetLocked (Variables|Default|GetDoor) false)
            (Utilities|IsValid (Variables|/Game/Blueprints/BP_Door.BP_Door_C|GetNavLink (Variables|Default|GetDoor))
              (:Is%20Valid
                (Class|NavLinkProxy|SetSmartLinkEnabled (Variables|/Game/Blueprints/BP_Door.BP_Door_C|GetNavLink (Variables|Default|GetDoor)) true))
              (:Is%20Not%20Valid
                _))
            (Variables|Default|SetDoor 0)
            (Audio|PlaySoundatLocation "/Game/Sounds/lock_creaking.lock_creaking" (Transformation|GetActorLocation) "0, 0, 0" 1.0 1.0 0.0 "/Game/Sounds/Attenuation/PhoneAtten.PhoneAtten" 0 0)
            (Variables|Default|SetUnlocked? true)
            (bind _asgame_instance_hnar (Utilities|Casting|CastToGameInstanceHNAR (Game|GetGameInstance)))
            (if (Utilities|Enum|Equal(Enum) _code "switch")
              (Variables|/Game/SaveData.SaveData_C|SetunlockedSilverKey (Variables|/Game/GameInstanceHNAR.GameInstanceHNAR_C|GetAs%20Save%20Data _asgame_instance_hnar) true)
              (Default|SavePuzzleData _asgame_instance_hnar :!label _label_2)
              (elif (Utilities|Enum|Equal(Enum) _code "shed2")
                (Variables|/Game/SaveData.SaveData_C|SetunlockedShedKey (Variables|/Game/GameInstanceHNAR.GameInstanceHNAR_C|GetAs%20Save%20Data _asgame_instance_hnar) true)
                (goto _label_2)
                (elif (Utilities|Enum|Equal(Enum) _code "blue")
                  (Variables|/Game/SaveData.SaveData_C|SetunlockedBlueKey (Variables|/Game/GameInstanceHNAR.GameInstanceHNAR_C|GetAs%20Save%20Data _asgame_instance_hnar) true)
                  (goto _label_2)
                  (elif (Utilities|Enum|Equal(Enum) _code "backroom")
                    (Variables|/Game/SaveData.SaveData_C|SetunlockedGreenKey (Variables|/Game/GameInstanceHNAR.GameInstanceHNAR_C|GetAs%20Save%20Data _asgame_instance_hnar) true)
                    (goto _label_2)
                    (elif (Utilities|Enum|Equal(Enum) _code "shed")
                      (Variables|/Game/SaveData.SaveData_C|SetunlockedShedDoor (Variables|/Game/GameInstanceHNAR.GameInstanceHNAR_C|GetAs%20Save%20Data _asgame_instance_hnar) true)
                      (goto _label_2)
                      (elif (Utilities|Enum|Equal(Enum) _code "lamproom")
                        (Variables|/Game/SaveData.SaveData_C|SetunlockedRedKey (Variables|/Game/GameInstanceHNAR.GameInstanceHNAR_C|GetAs%20Save%20Data _asgame_instance_hnar) true)
                        (goto _label_2)
                        (elif (Utilities|Enum|Equal(Enum) _code "exit_act2")
                          (Variables|/Game/SaveData.SaveData_C|SetunlockedBasementKey (Variables|/Game/GameInstanceHNAR.GameInstanceHNAR_C|GetAs%20Save%20Data _asgame_instance_hnar) true)
                          (goto _label_2))))))))))
        (else
          (Variables|/Game/Blueprints/BP_Door.BP_Door_C|SetLocked (Variables|Default|GetDoor) true)
          (goto _label Reset))))))

(event EventSetSocket
  (bind _asfirst_person_character (Utilities|Casting|CastToFirstPersonCharacter (Game|GetPlayerCharacter 0)))
  (Variables|Default|SetSocket (Variables|/Game/Blueprints/Characters/FirstPersonBP/Blueprints/FirstPersonCharacter.FirstPersonCharacter_C|GetLock _asfirst_person_character)))

(fn ConstructionScript
  (|CallParentFunction))