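; BP_Chair is a carryable chair the player can wedge against a closed door's ChairBlock to lock it.
; Use traces for an eligible door, removes the chair from inventory, snaps it to the door's Stool transform and registers it.
; NeighborKick pauses the AI for a kick animation, unlocks the door and launches the chair with a physics impulse.
; Tick re-enables the door's smart nav link and clears its reference once the chair is picked up.
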(event EventTick
  (params (DeltaSeconds :type Float%20%28single-precision%29))
  (bind _door (Variables|Default|GetDoor))
  (Utilities|IsValid _door
    (:Is%20Valid
      (if (== (Variables|/Game/Blueprints/BP_Door.BP_Door_C|GetSelectChair _door) self)
        (if (Variables|Default|GetIsPickedUp?)
          (Utilities|FlowControl|DoOnce false :!label _label
            (:Completed
              (Utilities|FlowControl|Delay 0.02)
              (Class|NavLinkProxy|SetSmartLinkEnabled (Variables|/Game/Blueprints/BP_Door.BP_Door_C|GetNavLink _door) true)
              (Utilities|FlowControl|Delay 0.1)
              (Variables|/Game/Blueprints/BP_Door.BP_Door_C|SetSelectChair _door 0)))
          (else
            (goto _label Reset)))))))

(event EventSetSocket
  (bind _asfirst_person_character (Utilities|Casting|CastToFirstPersonCharacter (Game|GetPlayerCharacter 0)))
  (Variables|Default|SetSocket (Variables|/Game/Blueprints/Characters/FirstPersonBP/Blueprints/FirstPersonCharacter.FirstPersonCharacter_C|GetStool _asfirst_person_character)))

(event EventNeighborKick
  (params (AI :type AI%20Object%20Reference))
  (bind _door (Variables|Default|GetDoor))
  (bind _charactermovement (Variables|/Script/Engine.Character|GetCharacterMovement AI))
  (Utilities|FlowControl|DoOnce false :!label _label
    (:Completed
      (Pawn|Components|CharacterMovement|SetMovementMode _charactermovement "MOVE_None" 0)
      (Default|PlayAnimAI AI "/Game/Neighbor/Animations/neighbour_lowpoly_Anim_rig_kick.neighbour_lowpoly_Anim_rig_kick" false)
      (Utilities|FlowControl|Delay 0.55)
      (Utilities|IsValid _door
        (:Is%20Valid
          (Physics|SetSimulatePhysics (Variables|Default|GetStaticMesh) true)
          (Variables|/Game/Blueprints/BP_Door.BP_Door_C|SetLocked _door false)
          (Variables|/Game/Blueprints/BP_Door.BP_Door_C|SetIsLockedWithChair? _door false))
        (:Is%20Not%20Valid
          _))
      (Physics|AddImpulse (Variables|Default|GetStaticMesh) (Variables|Default|GetKickImpulse) "None" true)
      (Utilities|FlowControl|Delay 0.81)
      (Pawn|Components|CharacterMovement|SetMovementMode _charactermovement "MOVE_Walking" 0)
      (Components|Animation|SetAnimationMode (Variables|/Script/Engine.Character|GetMesh AI) "AnimationBlueprint")
      (goto _label Reset))))

(event EventUse
  (bind _asfirst_person_character (Utilities|Casting|CastToFirstPersonCharacter (Game|GetPlayerCharacter 0)))
  (bind (_out_hit _return_value) (Default|Trace _asfirst_person_character "TraceTypeQuery3"))
  (if _return_value
    (bind _asbp_door (Utilities|Casting|CastToBP_Door (.HitActor (Collision|BreakHitResult _out_hit))))
    (bind _asbp_double_door (Utilities|Casting|CastToBP_DoubleDoor (.HitActor (Collision|BreakHitResult _out_hit)))
      (:then
        (if (not (Variables|/Game/Blueprints/BP_DoubleDoor.BP_DoubleDoor_C|GetOpen_1 _asbp_double_door))
          (if (Variables|/Game/Blueprints/BP_Door.BP_Door_C|GetCanLockDoorWithChair? _asbp_door) :!label _label
            (if (not (Variables|/Game/Blueprints/BP_Door.BP_Door_C|GetIsLockedWithChair? _asbp_door))
              (if (not (Variables|/Game/Blueprints/BP_Door.BP_Door_C|GetOpen _asbp_door))
                (if (== (.HitComponent (Collision|BreakHitResult _out_hit)) (Variables|/Game/Blueprints/BP_Door.BP_Door_C|GetChairBlock _asbp_door))
                  (Variables|Default|SetDoor _asbp_door)
                  (Utilities|Array|RemoveItem (Variables|/Game/Blueprints/Characters/FirstPersonBP/Blueprints/FirstPersonCharacter.FirstPersonCharacter_C|GetInventory _asfirst_person_character) self)
                  (Transformation|DetachFromActor "KeepRelative" "KeepRelative" "KeepWorld")
                  (Math|Integer|DecrementInt (Variables|/Game/Blueprints/Characters/FirstPersonBP/Blueprints/FirstPersonCharacter.FirstPersonCharacter_C|GetSelectedItem _asfirst_person_character)
                    (:%20%20
                      (Collision|SetCollisionEnabled (Variables|Default|GetStaticMesh) "QueryAndPhysics")
                      (Variables|Default|SetIsPickedUp? false)
                      (Transformation|SetActorLocationAndRotation (.location (Transformation|GetWorldTransform (Variables|/Game/Blueprints/BP_Door.BP_Door_C|GetStool _asbp_door))) (.rotation (Transformation|GetWorldTransform (Variables|/Game/Blueprints/BP_Door.BP_Door_C|GetStool _asbp_door))))
                      (Default|SetChair _asbp_door self)))))))))
      (:CastFailed
        (goto _label)))))

(fn ConstructionScript
  (|CallParentFunction))