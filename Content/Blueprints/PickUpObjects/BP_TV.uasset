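; Pickup TV the player can switch on and off, which lures the AI when turned on.
; Switching on plays static video on screen and spotlight with attached noise, reports a noise event and writes itself to the AI blackboard's ObjectRef.
; A TV starting on plays the Deadman video instead, tracked by NeighborTvOn for its separate shutdown.
; Hang disables physics, and OffHunt forces the static shutdown without the click sound.
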(event Custom|TurnOnOff
  (bind _returnvalue (Transformation|GetActorLocation))
  (bind _staticmesh (Variables|Default|GetStaticMesh))
  (bind _spotlight1 (Variables|Default|GetSpotLight1))
  (if (Variables|Default|GetOnOff)
    (Variables|Default|SetOnOff false)
    (Audio|PlaySoundatLocation "/Game/Sounds/TV_Turn_Off.TV_Turn_Off" _returnvalue "0, 0, 0" 1.0 1.0 0.0 "/Game/Sounds/Attenuation/FridgeAttenuation.FridgeAttenuation" 0 0)
    (if (Variables|Default|GetNeighbor%20tv%20on)
      (CallFunction|Off)
      (else
        (Rendering|Material|SetMaterial _staticmesh 0 "/Game/Materials/tv_monitor_dif_Mat.tv_monitor_dif_Mat")
        (Audio|Components|Audio|Stop (stale _returnvalue_2))
        (Rendering|SetVisibility _spotlight1 false false)))
    (else
      (Audio|PlaySoundatLocation "/Game/Sounds/TV_Turn_On.TV_Turn_On" _returnvalue "0, 0, 0" 1.0 1.0 0.0 "/Game/Sounds/Attenuation/FridgeAttenuation.FridgeAttenuation" 0 0)
      (Utilities|FlowControl|Delay 0.5)
      (Rendering|Material|SetMaterial _staticmesh 0 "/Game/Movies/tv_static_player_Video_Mat.tv_static_player_Video_Mat")
      (Media|MediaPlayer|OpenSource (Variables|Default|GetScreen) "/Game/Movies/tv_static.tv_static")
      (Media|MediaPlayer|OpenSource (Variables|Default|GetLight) "/Game/Movies/tv_static.tv_static")
      (Rendering|SetVisibility _spotlight1 true false)
      (bind _returnvalue_2 (Audio|SpawnSoundAttached "/Game/Sounds/TV_Noise_Cue.TV_Noise_Cue" _staticmesh "None" "0, 0, 0" "0, 0, 0" "KeepRelativeOffset" false 1.0 1.0 0.0 "/Game/Sounds/Attenuation/ItemAtten.ItemAtten" 0))
      (Variables|Default|SetOnOff true)
      (Class|AISenseHearing|ReportNoiseEvent (Transformation|GetWorldLocation (Variables|Default|GetStaticMesh)) 3.0 self 5e+02 "TV")
      (bind _returnvalue_3 (Actor|GetActorOfClass "/Game/Blueprints/Characters/AI2/AI.AI_C"))
      (AI|Components|Blackboard|SetValueasObject (AI|GetBlackboard _returnvalue_3) (Utilities|Name|MakeLiteralName "ObjectRef") self))))

(event Custom|On
  (bind _staticmesh (Variables|Default|GetStaticMesh))
  (Utilities|FlowControl|Delay 0.5)
  (Rendering|Material|SetMaterial _staticmesh 0 "/Game/Movies/tv_static_player_Video_Mat.tv_static_player_Video_Mat")
  (Media|MediaPlayer|OpenSource (Variables|Default|GetScreen) "/Game/Movies/deadman_tv_video.deadman_tv_video")
  (Media|MediaPlayer|OpenSource (Variables|Default|GetLight) "/Game/Movies/deadman_tv_video.deadman_tv_video")
  (bind _returnvalue (Audio|SpawnSoundAttached "/Game/Sounds/TV_sound_Cue.TV_sound_Cue" _staticmesh "None" "0, 0, 0" "0, 0, 0" "KeepRelativeOffset" false 1.0 1.0 0.0 "/Game/Sounds/Attenuation/RadioAtten.RadioAtten" 0))
  (Rendering|SetVisibility (Variables|Default|GetSpotLight1) true false)
  (Variables|Default|SetOnOff true)
  (Variables|Default|SetNeighbor%20tv%20on true))

(event Custom|Off
  (Rendering|Material|SetMaterial (Variables|Default|GetStaticMesh) 0 "/Game/Materials/tv_monitor_dif_Mat.tv_monitor_dif_Mat")
  (Audio|Components|Audio|Stop (stale Custom|On _returnvalue))
  (Rendering|SetVisibility (Variables|Default|GetSpotLight1) false false)
  (Variables|Default|SetOnOff false)
  (Variables|Default|SetNeighbor%20tv%20on false))

(event Custom|OffHunt
  (Variables|Default|SetOnOff false)
  (Rendering|Material|SetMaterial (Variables|Default|GetStaticMesh) 0 "/Game/Materials/tv_monitor_dif_Mat.tv_monitor_dif_Mat")
  (Audio|Components|Audio|Stop (stale Custom|TurnOnOff _returnvalue_2))
  (Rendering|SetVisibility (Variables|Default|GetSpotLight1) false false))

(event EventBeginPlay
  (Utilities|FlowControl|Sequence
    (:then_0
      (if (Variables|Default|GetOnOff)
        (CallFunction|On)))
    (:then_1
      (if (Variables|Default|GetHang?)
        (Physics|SetSimulatePhysics (Variables|Default|GetStaticMesh) false)))
    (:then_2
      (Utilities|FlowControl|Delay 1.0)
      (Variables|Default|SetStartTransform (Transformation|GetActorTransform)))))

(event Collision|EventActorBeginOverlap
  (params (OtherActor :type Actor%20Object%20Reference)))

(event EventTick
  (params (DeltaSeconds :type Float%20%28single-precision%29)))

(event EventSetSocket
  (bind _asfirst_person_character (Utilities|Casting|CastToFirstPersonCharacter (Game|GetPlayerCharacter 0)))
  (Variables|Default|SetSocket (Variables|/Game/Blueprints/Characters/FirstPersonBP/Blueprints/FirstPersonCharacter.FirstPersonCharacter_C|GetTV _asfirst_person_character)))

(event EventInteract
  (bind _returnvalue (Transformation|GetActorLocation))
  (bind _staticmesh (Variables|Default|GetStaticMesh))
  (bind _spotlight1 (Variables|Default|GetSpotLight1))
  (if (Variables|Default|GetOnOff)
    (Variables|Default|SetOnOff false)
    (Audio|PlaySoundatLocation "/Game/Sounds/TV_Turn_Off.TV_Turn_Off" _returnvalue "0, 0, 0" 1.0 1.0 0.0 "/Game/Sounds/Attenuation/FridgeAttenuation.FridgeAttenuation" 0 0)
    (if (Variables|Default|GetNeighbor%20tv%20on)
      (CallFunction|Off)
      (else
        (Rendering|Material|SetMaterial _staticmesh 0 "/Game/Materials/tv_monitor_dif_Mat.tv_monitor_dif_Mat")
        (Audio|Components|Audio|Stop (stale _returnvalue_2))
        (Rendering|SetVisibility _spotlight1 false false)))
    (else
      (Audio|PlaySoundatLocation "/Game/Sounds/TV_Turn_On.TV_Turn_On" _returnvalue "0, 0, 0" 1.0 1.0 0.0 "/Game/Sounds/Attenuation/FridgeAttenuation.FridgeAttenuation" 0 0)
      (Utilities|FlowControl|Delay 0.5)
      (Rendering|Material|SetMaterial _staticmesh 0 "/Game/Movies/tv_static_player_Video_Mat.tv_static_player_Video_Mat")
      (Media|MediaPlayer|OpenSource (Variables|Default|GetScreen) "/Game/Movies/tv_static.tv_static")
      (Media|MediaPlayer|OpenSource (Variables|Default|GetLight) "/Game/Movies/tv_static.tv_static")
      (Rendering|SetVisibility _spotlight1 true false)
      (bind _returnvalue_2 (Audio|SpawnSoundAttached "/Game/Sounds/TV_Noise_Cue.TV_Noise_Cue" _staticmesh "None" "0, 0, 0" "0, 0, 0" "KeepRelativeOffset" false 1.0 1.0 0.0 "/Game/Sounds/Attenuation/ItemAtten.ItemAtten" 0))
      (Variables|Default|SetOnOff true)
      (Class|AISenseHearing|ReportNoiseEvent (Transformation|GetWorldLocation (Variables|Default|GetStaticMesh)) 3.0 self 5e+02 "TV")
      (bind _returnvalue_3 (Actor|GetActorOfClass "/Game/Blueprints/Characters/AI2/AI.AI_C"))
      (AI|Components|Blackboard|SetValueasObject (AI|GetBlackboard _returnvalue_3) (Utilities|Name|MakeLiteralName "ObjectRef") self))))

(fn ConstructionScript
  (|CallParentFunction))