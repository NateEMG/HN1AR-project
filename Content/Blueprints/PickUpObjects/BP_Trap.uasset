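; Mantrap pickup that Interact toggles between open and closed, and that can only be picked up when closed.
; An open trap immobilises the player, rolls a random press count and alerts the AI through a blackboard object and noise event.
; A second box lets non-held, non-trap interactables spring it with the same alert.
; It also catches the AI in one specific state, blocking movement and catching until its trapped animation ends.
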(event OnComponentBeginOverlap(Box)
  (params (OverlappedComponent :type Primitive%20Component%20Object%20Reference) (OtherActor :type Actor%20Object%20Reference) (OtherComp :type Primitive%20Component%20Object%20Reference) (OtherBodyIndex :type Integer) (bFromSweep :type Boolean) (SweepResult :type Hit%20Result%20Structure%20%28by%20ref%29))
  (bind _self self)
  (bind _staticmesh (Variables|Default|GetStaticMesh))
  (bind _ai (Variables|Default|GetAI))
  (bind _returnvalue (Transformation|GetWorldLocation _staticmesh))
  (bind _asfirst_person_character (Utilities|Casting|CastToFirstPersonCharacter OtherActor))
  (if (not (Variables|/Game/Blueprints/Characters/FirstPersonBP/Blueprints/FirstPersonCharacter.FirstPersonCharacter_C|GetIsTrapped _asfirst_person_character))
    (Variables|Default|SetAs%20First%20Person%20Character _asfirst_person_character)
    (if (Variables|Default|GetIsOpen)
      (Variables|/Game/Blueprints/Characters/FirstPersonBP/Blueprints/FirstPersonCharacter.FirstPersonCharacter_C|SetTrapRef _asfirst_person_character self)
      (Pawn|Components|CharacterMovement|DisableMovement (Variables|/Script/Engine.Character|GetCharacterMovement _asfirst_person_character))
      (Components|StaticMesh|SetStaticMesh _staticmesh "/Game/Objects/Meshes/trap_closed_a4.trap_closed_a4")
      (Audio|PlaySoundatLocation "/Game/Sounds/mantrap.mantrap" _returnvalue "0, 0, 0" 1.0 1.0 0.0 "/Game/Sounds/Attenuation/NeighborVoiceAtten.NeighborVoiceAtten" 0 0)
      (Utilities|FlowControl|Sequence
        (:then_0
          (AI|Components|Blackboard|SetValueasObject (AI|GetBlackboard _ai) (Utilities|Name|MakeLiteralName "ObjectRef") _self)
          (if (Variables|/Game/Blueprints/Characters/AI2/AI.AI_C|GetCanHear _ai)
            (Class|AISenseHearing|ReportNoiseEvent _returnvalue 3.0 _self 1e+03 "Trap")))
        (:then_1
          (Variables|Default|SetPressesNeeded (Math|Conversions|ToFloat(Integer) (Math|Random|RandomIntegerinRange 7 13)))
          (Variables|/Game/Blueprints/Characters/FirstPersonBP/Blueprints/FirstPersonCharacter.FirstPersonCharacter_C|SetIsTrapped _asfirst_person_character true))))))

(event OnComponentBeginOverlap(Box1)
  (params (OverlappedComponent :type Primitive%20Component%20Object%20Reference) (OtherActor :type Actor%20Object%20Reference) (OtherComp :type Primitive%20Component%20Object%20Reference) (OtherBodyIndex :type Integer) (bFromSweep :type Boolean) (SweepResult :type Hit%20Result%20Structure%20%28by%20ref%29))
  (bind _self self)
  (bind _staticmesh (Variables|Default|GetStaticMesh))
  (bind _returnvalue (Transformation|GetWorldLocation _staticmesh))
  (bind _asbp_interactable (Utilities|Casting|CastToBP_Interactable OtherActor)
    (:then
      (if (== OtherComp (Variables|/Game/Blueprints/PickUpObjects/BP_Interactable.BP_Interactable_C|GetStaticMesh _asbp_interactable))
        (if (not (Utilities|String|Contains (Utilities|GetDisplayName OtherActor) "Trap"))
          (if (Variables|Default|GetIsOpen)
            (if (not (Variables|/Game/Blueprints/PickUpObjects/BP_Interactable.BP_Interactable_C|GetIsPickedUp? _asbp_interactable))
              (Components|StaticMesh|SetStaticMesh _staticmesh "/Game/Objects/Meshes/trap_closed_a4.trap_closed_a4")
              (Audio|PlaySoundatLocation "/Game/Sounds/mantrap.mantrap" _returnvalue "0, 0, 0" 1.0 1.0 0.0 "/Game/Sounds/Attenuation/NeighborVoiceAtten.NeighborVoiceAtten" 0 0)
              (AI|Components|Blackboard|SetValueasObject (AI|GetBlackboard (Variables|Default|GetAI)) (Utilities|Name|MakeLiteralName "ObjectRef") _self)
              (Class|AISenseHearing|ReportNoiseEvent _returnvalue 3.0 _self 1e+03 "Trap")
              (Variables|Default|SetIsOpen false)
              (Variables|Default|SetCanPickUp? true))))))
    (:CastFailed
      (bind _asai (Utilities|Casting|CastToAI OtherActor))
      (bind _output_get (Variables|Default|SetAI _asai))
      (if (not (Variables|/Game/Blueprints/Characters/AI2/AI.AI_C|GetIsTrapped _output_get))
        (if (Variables|Default|GetIsOpen)
          (if (Utilities|Enum|Equal(Enum) (Variables|/Game/Blueprints/Characters/AI2/AI.AI_C|GetCurrentState _output_get) "NewEnumerator4")
            (Variables|/Game/Blueprints/Characters/AI2/AI.AI_C|SetIsTrapped _output_get true)
            (Utilities|FlowControl|Delay 0.07)
            (Components|StaticMesh|SetStaticMesh (Variables|Default|GetStaticMesh) "/Game/Objects/Meshes/trap_closed_a4.trap_closed_a4")
            (Audio|PlaySoundatLocation "/Game/Sounds/mantrap.mantrap" (Transformation|GetWorldLocation (Variables|Default|GetStaticMesh)) "0, 0, 0" 1.0 1.0 0.0 "/Game/Sounds/Attenuation/NeighborVoiceAtten.NeighborVoiceAtten" 0 0)
            (Variables|Default|SetIsOpen false)
            (Variables|Default|SetCanPickUp? true)
            (Pawn|Components|CharacterMovement|DisableMovement (Variables|/Script/Engine.Character|GetCharacterMovement _output_get))
            (Variables|/Game/Blueprints/Characters/AI2/AI.AI_C|SetCanCatch _output_get false)
            (bind _anim_length (Default|PlayAnimAI _output_get "/Game/Neighbor/Animations/neighbour_lowpoly_Anim_rig_trap.neighbour_lowpoly_Anim_rig_trap" false))
            (Utilities|FlowControl|Delay _anim_length)
            (Components|Animation|SetAnimationMode (Variables|/Script/Engine.Character|GetMesh _output_get) "AnimationBlueprint")
            (Pawn|Components|CharacterMovement|SetMovementMode (Variables|/Script/Engine.Character|GetCharacterMovement _output_get) "MOVE_Walking" 0)
            (Variables|/Game/Blueprints/Characters/AI2/AI.AI_C|SetCanCatch _output_get true)
            (Variables|/Game/Blueprints/Characters/AI2/AI.AI_C|SetIsTrapped _output_get false)))))))

(event Custom|SetOpen
  (bind _staticmesh (Variables|Default|GetStaticMesh))
  (if (Variables|Default|GetIsOpen)
    (Components|StaticMesh|SetStaticMesh _staticmesh "/Game/Objects/Meshes/trap_closed_a4.trap_closed_a4")
    (Variables|Default|SetIsOpen false)
    (Variables|Default|SetCanPickUp? true)
    (else
      (Components|StaticMesh|SetStaticMesh _staticmesh "/Game/Objects/Meshes/trap_a4.trap_a4")
      (Variables|Default|SetIsOpen true)
      (Variables|Default|SetCanPickUp? false))))

(event Custom|CustomTick
  (Utilities|Time|SetTimerbyEvent (delegate Custom|CustomTick) 0.1 true)
  (if (Variables|/Game/Blueprints/Characters/FirstPersonBP/Blueprints/FirstPersonCharacter.FirstPersonCharacter_C|GetIsTrapped (Variables|Default|GetAs%20First%20Person%20Character))
    _))

(event EventBeginPlay
  (bind _staticmesh (Variables|Default|GetStaticMesh))
  (|CallParentFunction)
  (bind _asfirst_person_character (Utilities|Casting|CastToFirstPersonCharacter (Game|GetPlayerCharacter 0)))
  (Variables|Default|SetAs%20First%20Person%20Character _asfirst_person_character)
  (bind _returnvalue (Actor|GetActorOfClass "/Game/Blueprints/Characters/AI2/AI.AI_C"))
  (Variables|Default|SetAI _returnvalue)
  (if (Variables|Default|GetIsOpen)
    (Components|StaticMesh|SetStaticMesh _staticmesh "/Game/Objects/Meshes/trap_a4.trap_a4")
    (Variables|Default|SetCanPickUp? false)
    (else
      (Components|StaticMesh|SetStaticMesh _staticmesh "/Game/Objects/Meshes/trap_closed_a4.trap_closed_a4")
      (Variables|Default|SetCanPickUp? true))))

(event EventSetSocket
  (bind _asfirst_person_character (Utilities|Casting|CastToFirstPersonCharacter (Game|GetPlayerCharacter 0)))
  (Variables|Default|SetSocket (Variables|/Game/Blueprints/Characters/FirstPersonBP/Blueprints/FirstPersonCharacter.FirstPersonCharacter_C|GetTrap _asfirst_person_character)))

(event EventInteract
  (bind _staticmesh (Variables|Default|GetStaticMesh))
  (if (not (Variables|/Game/Blueprints/Characters/FirstPersonBP/Blueprints/FirstPersonCharacter.FirstPersonCharacter_C|GetIsTrapped (Variables|Default|GetAs%20First%20Person%20Character)))
    (if (Variables|Default|GetIsOpen)
      (Components|StaticMesh|SetStaticMesh _staticmesh "/Game/Objects/Meshes/trap_closed_a4.trap_closed_a4")
      (Variables|Default|SetIsOpen false)
      (Variables|Default|SetCanPickUp? true)
      (else
        (Components|StaticMesh|SetStaticMesh _staticmesh "/Game/Objects/Meshes/trap_a4.trap_a4")
        (Variables|Default|SetIsOpen true)
        (Variables|Default|SetCanPickUp? false)))))

(fn ConstructionScript
  (|CallParentFunction))