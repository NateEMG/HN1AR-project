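; BP_Milk is a drinkable milk pickup that speeds up game time when used.
; On BeginPlay it runs the parent logic and sets Socket to the first-person character's Milk member.
; Use calls Drop, plays a slurp sound, then after a short delay runs a "slomo" console command to accelerate time and destroys the actor.
; Nothing in this Blueprint restores normal speed.
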(event EventBeginPlay
  (|CallParentFunction)
  (bind _asfirst_person_character (Utilities|Casting|CastToFirstPersonCharacter (Game|GetPlayerCharacter 0)))
  (Variables|Default|SetSocket (Variables|/Game/Blueprints/Characters/FirstPersonBP/Blueprints/FirstPersonCharacter.FirstPersonCharacter_C|GetMilk _asfirst_person_character)))

(event Collision|EventActorBeginOverlap
  (params (OtherActor :type Actor%20Object%20Reference)))

(event EventTick
  (params (DeltaSeconds :type Float%20%28single-precision%29)))

(event EventUse
  (CallFunction|Drop)
  (Audio|PlaySound2D "/Game/Sounds/slurp.slurp" 1.0 1.0 0.0 0 0)
  (Utilities|FlowControl|Delay 0.4)
  (Development|ExecuteConsoleCommand "slomo 5" (Game|GetPlayerController 0))
  (Actor|DestroyActor))

(fn ConstructionScript
  (|CallParentFunction))