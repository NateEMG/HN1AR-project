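; BP_Jackhammer is a pickup tool that removes bricks from a brick wall when used.
; SetSocket takes the Jackhammer socket from the first-person character.
; Use calls the character's Visibility trace and, on a hit BP_BrickWall, passes the hit component to RemoveBrick unless it is the wall's Fault component.
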(event EventBeginPlay
  (|CallParentFunction) ; This node is disabled and will not be called.\nDrag off pins to build functionality.
)

(event Collision|EventActorBeginOverlap
  (params (OtherActor :type Actor%20Object%20Reference)))

(event EventTick
  (params (DeltaSeconds :type Float%20%28single-precision%29)))

(event EventUse
  (bind _asfirst_person_character (Utilities|Casting|CastToFirstPersonCharacter (Game|GetPlayerCharacter 0)))
  (bind (_out_hit _return_value) (Default|Trace _asfirst_person_character "TraceTypeQuery1"))
  (if _return_value
    (bind _asbp_brick_wall (Utilities|Casting|CastToBP_BrickWall (.HitActor (Collision|BreakHitResult _out_hit))))
    (if (not (== (Variables|/Game/Blueprints/PuzzleBPs/BP_BrickWall.BP_BrickWall_C|Getfault _asbp_brick_wall) (.HitComponent (Collision|BreakHitResult _out_hit))))
      (Default|RemoveBrick _asbp_brick_wall (.HitComponent (Collision|BreakHitResult _out_hit))))))

(event EventSetSocket
  (bind _asfirst_person_character (Utilities|Casting|CastToFirstPersonCharacter (Game|GetPlayerCharacter 0)))
  (Variables|Default|SetSocket (Variables|/Game/Blueprints/Characters/FirstPersonBP/Blueprints/FirstPersonCharacter.FirstPersonCharacter_C|GetJackhammer _asfirst_person_character)))

(fn ConstructionScript
  (|CallParentFunction))