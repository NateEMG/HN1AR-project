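; Base physics prop that can be picked up, dropped or thrown, with empty interact, use and socket events.
; Pickup and drop toggle physics and collision; props flagged Hang start with physics off.
; Hard hits play a sound, and player-thrown ones also report AI noise, set the neighbor AI's blackboard ObjectRef and increment its fall count.
; AI contact can trigger a timed kick animation that launches the prop forward and upward.
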(event OnComponentHit(StaticMesh)
  (params (HitComponent :type Primitive%20Component%20Object%20Reference) (OtherActor :type Actor%20Object%20Reference) (OtherComp :type Primitive%20Component%20Object%20Reference) (NormalImpulse :type Vector :default "0, 0, 0") (Hit :type Hit%20Result%20Structure%20%28by%20ref%29))
  (bind _asai (Utilities|Casting|CastToAI OtherActor))
  (if (Variables|Default|GetCanKick?)
    (if (Variables|/Game/Blueprints/Characters/AI2/AI.AI_C|GetCanAIKick _asai)
      (if (not (Utilities|Enum|Equal(Enum) (Class|SkeletalMeshComponent|GetAnimationMode (Variables|/Script/Engine.Character|GetMesh _asai)) "AnimationSingleNode"))
        (CallFunction|NeighborKick _asai)))))

(event Custom|NeighborKick
  (params (AI :type AI%20Object%20Reference))
  (bind _charactermovement (Variables|/Script/Engine.Character|GetCharacterMovement AI))
  (Utilities|FlowControl|DoOnce false :!label _label
    (:Completed
      (Utilities|FlowControl|Delay 0.2)
      (Pawn|Components|CharacterMovement|SetMovementMode _charactermovement "MOVE_None" 0)
      (Default|PlayAnimAI AI "/Game/Neighbor/Animations/neighbour_lowpoly_Anim_rig_kick.neighbour_lowpoly_Anim_rig_kick" false)
      (Utilities|FlowControl|Delay 0.55)
      (Physics|AddImpulse (Variables|Default|GetStaticMesh) (* (Math|Vector|RotateVector (Transformation|GetActorForwardVector AI) (Math|Vector|RotatorfromAxisandAngle (Math|Vector|NegateVector (Transformation|GetActorRightVector AI)) 3e+01)) 1.5e+03) "None" true)
      (Utilities|FlowControl|Delay 0.81)
      (Pawn|Components|CharacterMovement|SetMovementMode _charactermovement "MOVE_Walking" 0)
      (Components|Animation|SetAnimationMode (Variables|/Script/Engine.Character|GetMesh AI) "AnimationBlueprint")
      (goto _label Reset))))

(event Custom|Pick%20Up
  (bind _staticmesh (Variables|Default|GetStaticMesh))
  (Physics|SetSimulatePhysics _staticmesh false)
  (Collision|SetCollisionEnabled _staticmesh "NoCollision")
  (Variables|Default|SetIsPickedUp? true)
  (Audio|PlaySoundatLocation (Variables|Default|GetPick%20Up%20Sound) (Transformation|GetWorldLocation _staticmesh) "0, 0, 0" 1.0 1.0 0.0 0 0 0))

(event Custom|Interact)

(event Custom|Drop
  (bind _staticmesh (Variables|Default|GetStaticMesh))
  (Physics|SetSimulatePhysics _staticmesh true)
  (Collision|SetCollisionEnabled _staticmesh "QueryAndPhysics")
  (Variables|Default|SetIsPickedUp? false))

(event Custom|Use)

(event Custom|SetSocket)

(event Custom|HitEvent
  (params (SelfActor :type Actor%20Object%20Reference) (OtherActor :type Actor%20Object%20Reference) (NormalImpulse :type Vector) (Hit :type Hit%20Result%20Structure%20%28by%20ref%29))
  (if (> (Math|Vector|VectorLength NormalImpulse) (Variables|Default|GetImpulse%20Threshold))
    (if (Variables|Default|GetPlayerThrown?)
      (Class|AISenseHearing|ReportNoiseEvent (Transformation|GetActorLocation) 3.0 self 3e+02 "ThrownItem")
      (Development|PrintString "Thrown Item Loudly" true true "(R=0.000000,G=1.000000,B=0.707907,A=1.000000)")
      (bind _returnvalue (Actor|GetActorOfClass "/Game/Blueprints/Characters/AI2/AI.AI_C"))
      (Utilities|IsValid _returnvalue
        (:Is%20Valid
          (AI|Components|Blackboard|SetValueasObject (AI|GetBlackboard _returnvalue) (Utilities|Name|MakeLiteralName "ObjectRef") self)
          (Math|Integer|IncrementInt (Variables|/Game/Blueprints/Characters/AI2/AI.AI_C|GetItemFallCount _returnvalue)
            (:%20%20
              _)))
        (:Is%20Not%20Valid
          _))
      (Variables|Default|SetPlayerThrown? false))
    (Utilities|FlowControl|DoOnce false :!label _label
      (:Completed
        (Audio|PlaySoundatLocation (Variables|Default|GetHit%20Sound) (.impactpoint Hit) "0, 0, 0" 1.0 1.0 0.0 0 0 0)
        (Utilities|FlowControl|Delay 0.1)
        (goto _label Reset)))))

(event Custom|SetNeighborSocket)

(event EventBeginPlay
  (bind _staticmesh (Variables|Default|GetStaticMesh))
  (Utilities|FlowControl|Sequence
    (:then_0
      (Class|PrimitiveComponent|SetNotifyRigidBodyCollision (Variables|Default|GetStaticMesh) true)
      (Collision|BindEventtoOnActorHit (delegate Custom|HitEvent)))
    (:then_1
      (Variables|Default|SetIsPickedUp? false))
    (:then_2
      (if (Variables|Default|GetHang?)
        (Physics|SetSimulatePhysics _staticmesh false)
        (else
          (Physics|SetSimulatePhysics _staticmesh true))))
    (:then_3
      (Utilities|FlowControl|Delay 1.0)
      (Variables|Default|SetStartTransform (Transformation|GetActorTransform)))))

(fn ConstructionScript)