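; BP_Board1 is a breakable board that can become a pick-up object once broken.
; On BeginPlay it runs the parent logic, hides its skeletal mesh, takes the FirstPersonCharacter's Board as its Socket and disables pick-up.
; The break event plays a sound at the board's location, then, only once, either destroys the actor if Dissapear is set or enables static mesh physics and pick-up.
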(event Custom|break
  (Audio|PlaySoundatLocation "/Game/Sounds/break_board.break_board" (Transformation|GetActorLocation) "0, 0, 0" 1.0 1.0 0.0 "/Game/Sounds/Attenuation/PhoneAtten.PhoneAtten" 0 0)
  (Utilities|FlowControl|DoOnce false
    (:Completed
      (if (Variables|Default|GetDissapear)
        (Actor|DestroyActor)
        (else
          (Physics|SetSimulatePhysics (Variables|Default|GetStaticMesh) true)
          (Variables|Default|SetCanPickUp? true))))))

(event EventBeginPlay
  (|CallParentFunction)
  (Rendering|SetVisibility (Variables|Default|GetSkeletalMesh) false false)
  (bind _asfirst_person_character (Utilities|Casting|CastToFirstPersonCharacter (Game|GetPlayerCharacter 0)))
  (Variables|Default|SetSocket (Variables|/Game/Blueprints/Characters/FirstPersonBP/Blueprints/FirstPersonCharacter.FirstPersonCharacter_C|GetBoard _asfirst_person_character))
  (Variables|Default|SetCanPickUp? false))

(event EventTick
  (params (DeltaSeconds :type Float%20%28single-precision%29)))

(fn ConstructionScript
  (|CallParentFunction))