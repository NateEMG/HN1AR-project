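; BP_Binoculars is a usable binoculars object that zooms the first-person camera and shows a binocular overlay.
; BeginPlay stores the character's Binoculars reference as Socket and adds a hidden W_BinocularView widget to the viewport.
; Use narrows the camera's field of view and reveals the overlay.
; Tick polls mouse input, restoring the wider view and hiding the overlay on left-button release, or left press while right is held.
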(event EventBeginPlay
  (bind _asfirst_person_character (Utilities|Casting|CastToFirstPersonCharacter (Game|GetPlayerCharacter 0)))
  (Variables|Default|SetSocket (Variables|/Game/Blueprints/Characters/FirstPersonBP/Blueprints/FirstPersonCharacter.FirstPersonCharacter_C|GetBinoculars _asfirst_person_character))
  (bind _returnvalue (UserInterface|CreateWidget "/Game/Blueprints/UI/W_BinocularView.W_BinocularView_C"))
  (bind _output_get (Variables|Default|SetBinocularView _returnvalue))
  (UserInterface|Viewport|AddtoViewport _output_get 0)
  (Widget|SetVisibility _output_get "Hidden"))

(event Collision|EventActorBeginOverlap
  (params (OtherActor :type Actor%20Object%20Reference)))

(event EventTick
  (params (DeltaSeconds :type Float%20%28single-precision%29))
  (bind _returnvalue (Game|GetPlayerController 0))
  (Utilities|FlowControl|Sequence
    (:then_0
      (if (Class|PlayerController|WasInputKeyJustReleased _returnvalue "LeftMouseButton")
        (bind _asfirst_person_character (Utilities|Casting|CastToFirstPersonCharacter (Game|GetPlayerCharacter 0) :!label _label))
        (Camera|SetFieldOfView (Variables|/Game/Blueprints/Characters/FirstPersonBP/Blueprints/FirstPersonCharacter.FirstPersonCharacter_C|GetFirstPersonCamera _asfirst_person_character) 1e+02)
        (Widget|SetVisibility (Variables|Default|GetBinocularView) "Hidden")))
    (:then_1
      (if (Game|Player|IsInputKeyDown _returnvalue "RightMouseButton")
        (if (Game|Player|WasInputKeyJustPressed _returnvalue "LeftMouseButton")
          (goto _label))))))

(event EventUse
  (bind _asfirst_person_character (Utilities|Casting|CastToFirstPersonCharacter (Game|GetPlayerCharacter 0)))
  (Camera|SetFieldOfView (Variables|/Game/Blueprints/Characters/FirstPersonBP/Blueprints/FirstPersonCharacter.FirstPersonCharacter_C|GetFirstPersonCamera _asfirst_person_character) 2e+01)
  (Widget|SetVisibility (Variables|Default|GetBinocularView) "Visible"))

(fn ConstructionScript
  (|CallParentFunction))