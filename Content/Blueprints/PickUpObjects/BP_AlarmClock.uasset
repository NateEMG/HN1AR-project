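; Alarm clock pickup that acts as a timed noise lure for the AI, held at the player's Ball socket.
; Use toggles the ticking audio unless right mouse is held or the clock is ringing.
; When ticking audio finishes, it plays the alarm; if the AI can hear, it reports a noise event and sets itself as the blackboard's ObjectRef.
; Only that hearing branch clears the ticking and ringing flags, after a delay.
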(event OnAudioFinished(Audio)
  (bind _returnvalue (Transformation|GetActorLocation))
  (if (Variables|Default|GetIsTicking)
    (Variables|Default|SetIsRinging true)
    (Audio|PlaySoundatLocation "/Game/Sounds/alarm-clock.alarm-clock" _returnvalue "0, 0, 0" 1.0 1.0 0.0 "/Game/Sounds/Attenuation/DoorSoundAttenuation.DoorSoundAttenuation" 0 0)
    (bind _returnvalue_2 (Actor|GetActorOfClass "/Game/Blueprints/Characters/AI2/AI.AI_C"))
    (if (Variables|/Game/Blueprints/Characters/AI2/AI.AI_C|GetCanHear _returnvalue_2)
      (Class|AISenseHearing|ReportNoiseEvent _returnvalue 5.0 self 8e+02 "Alarm")
      (bind _returnvalue_3 (Actor|GetActorOfClass "/Game/Blueprints/Characters/AI2/AI.AI_C"))
      (AI|Components|Blackboard|SetValueasObject (AI|GetBlackboard _returnvalue_3) (Utilities|Name|MakeLiteralName "ObjectRef") self)
      (Utilities|FlowControl|Delay 6.328)
      (Variables|Default|SetIsTicking false)
      (Variables|Default|SetIsRinging false))))

(event EventBeginPlay
  (|CallParentFunction)
  (Audio|Components|Audio|Stop (Variables|Default|GetAudio)))

(event Collision|EventActorBeginOverlap
  (params (OtherActor :type Actor%20Object%20Reference)))

(event EventTick
  (params (DeltaSeconds :type Float%20%28single-precision%29)))

(event EventSetSocket
  (bind _asfirst_person_character (Utilities|Casting|CastToFirstPersonCharacter (Game|GetPlayerCharacter 0)))
  (Variables|Default|SetSocket (Variables|/Game/Blueprints/Characters/FirstPersonBP/Blueprints/FirstPersonCharacter.FirstPersonCharacter_C|GetBall _asfirst_person_character)))

(event EventUse
  (bind _audio (Variables|Default|GetAudio))
  (if (not (Game|Player|IsInputKeyDown (Game|GetPlayerController 0) "RightMouseButton"))
    (if (not (Variables|Default|GetIsRinging))
      (Utilities|FlowControl|FlipFlop
        (:A
          (Audio|Components|Audio|Play _audio 0.0)
          (Variables|Default|SetIsTicking true))
        (:B
          (Variables|Default|SetIsTicking false)
          (Audio|Components|Audio|Stop _audio))))))

(fn ConstructionScript
  (|CallParentFunction))