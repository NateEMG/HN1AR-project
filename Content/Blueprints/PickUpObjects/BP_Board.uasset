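; Pickup board that can bar an assigned door until it breaks loose.
; On BeginPlay it hides its skeletal mesh, takes the player's Board socket and, if a door is assigned, disables pickup and optionally locks it.
; Tick keeps the door locked until the static mesh simulates physics, then unlocks and releases it with a break sound.
; The board's Tag selects which of four unlocked flags is written to the puzzle save.
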(event EventBeginPlay
  (bind _door (Variables|Default|GetDoor))
  (|CallParentFunction)
  (Rendering|SetVisibility (Variables|Default|GetSkeletalMesh) false false)
  (bind _asfirst_person_character (Utilities|Casting|CastToFirstPersonCharacter (Game|GetPlayerCharacter 0)))
  (Variables|Default|SetSocket (Variables|/Game/Blueprints/Characters/FirstPersonBP/Blueprints/FirstPersonCharacter.FirstPersonCharacter_C|GetBoard _asfirst_person_character))
  (Utilities|IsValid _door
    (:Is%20Valid
      (Variables|Default|SetCanPickUp? false)
      (if (Variables|Default|GetLockDoor?)
        (Variables|/Game/Blueprints/BP_Door.BP_Door_C|SetLocked _door true)
        (Variables|Default|SetIsLocked? true)))))

(event EventTick
  (params (DeltaSeconds :type Float%20%28single-precision%29))
  (bind _tag (Variables|Default|GetTag))
  (Utilities|IsValid (Variables|Default|GetDoor)
    (:Is%20Valid
      (if (Physics|IsSimulatingPhysics (Variables|Default|GetStaticMesh) "None")
        (Utilities|FlowControl|DoOnce false :!label _label
          (:Completed
            (Variables|/Game/Blueprints/BP_Door.BP_Door_C|SetLocked (Variables|Default|GetDoor) false)
            (Variables|Default|SetDoor 0)
            (Audio|PlaySoundatLocation "/Game/Sounds/break_board.break_board" (Transformation|GetActorLocation) "0, 0, 0" 1.0 1.0 0.0 "/Game/Sounds/Attenuation/PhoneAtten.PhoneAtten" 0 0)
            (if (Utilities|Enum|Equal(Enum) _tag "1")
              (Variables|/Game/SaveData.SaveData_C|SetunlockedBoard_1 (Variables|/Game/GameInstanceHNAR.GameInstanceHNAR_C|GetAs%20Save%20Data (Variables|/Game/Blueprints/Characters/FirstPersonBP/Blueprints/FirstPersonCharacter.FirstPersonCharacter_C|GetAs%20Game%20Instance%20HNAR (stale EventBeginPlay _asfirst_person_character))) true)
              (Default|SavePuzzleData (Variables|/Game/Blueprints/Characters/FirstPersonBP/Blueprints/FirstPersonCharacter.FirstPersonCharacter_C|GetAs%20Game%20Instance%20HNAR (stale EventBeginPlay _asfirst_person_character)) :!label _label_2)
              (elif (Utilities|Enum|Equal(Enum) _tag "2")
                (Variables|/Game/SaveData.SaveData_C|SetunlockedBoard_2 (Variables|/Game/GameInstanceHNAR.GameInstanceHNAR_C|GetAs%20Save%20Data (Variables|/Game/Blueprints/Characters/FirstPersonBP/Blueprints/FirstPersonCharacter.FirstPersonCharacter_C|GetAs%20Game%20Instance%20HNAR (stale EventBeginPlay _asfirst_person_character))) true)
                (goto _label_2)
                (elif (Utilities|Enum|Equal(Enum) _tag "3")
                  (Variables|/Game/SaveData.SaveData_C|SetunlockedBoard_3 (Variables|/Game/GameInstanceHNAR.GameInstanceHNAR_C|GetAs%20Save%20Data (Variables|/Game/Blueprints/Characters/FirstPersonBP/Blueprints/FirstPersonCharacter.FirstPersonCharacter_C|GetAs%20Game%20Instance%20HNAR (stale EventBeginPlay _asfirst_person_character))) true)
                  (goto _label_2)
                  (elif (Utilities|Enum|Equal(Enum) _tag "4")
                    (Variables|/Game/SaveData.SaveData_C|SetunlockedBoard_4 (Variables|/Game/GameInstanceHNAR.GameInstanceHNAR_C|GetAs%20Save%20Data (Variables|/Game/Blueprints/Characters/FirstPersonBP/Blueprints/FirstPersonCharacter.FirstPersonCharacter_C|GetAs%20Game%20Instance%20HNAR (stale EventBeginPlay _asfirst_person_character))) true)
                    (goto _label_2)))))))
        (else
          (Variables|/Game/Blueprints/BP_Door.BP_Door_C|SetLocked (Variables|Default|GetDoor) true)
          (goto _label Reset))))))

(fn ConstructionScript
  (|CallParentFunction))