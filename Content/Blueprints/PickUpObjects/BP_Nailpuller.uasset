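; Nailpuller pickup tool that lets the player pry loose or break boards.
; SetSocket takes the character's Nailpuller socket, and Use traces from the character for a board's Cube component.
; On a hit, input is disabled while a skeletal mesh replaces the static one at the board and plays an animation.
; Timed delays release BP_Board to physics as pickable or call Break on BP_Board1, then restore the tool and input.
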(event EventSetSocket
  (bind _asfirst_person_character (Utilities|Casting|CastToFirstPersonCharacter (Game|GetPlayerCharacter 0)))
  (Variables|Default|SetSocket (Variables|/Game/Blueprints/Characters/FirstPersonBP/Blueprints/FirstPersonCharacter.FirstPersonCharacter_C|GetNailpuller _asfirst_person_character)))

(event EventUse
  (bind _returnvalue (Game|GetPlayerController 0))
  (bind _skeletalmesh (Variables|Default|GetSkeletalMesh))
  (bind _staticmesh (Variables|Default|GetStaticMesh))
  (bind _skeletalmesh_2 (Variables|Default|GetSkeletalMesh))
  (bind _staticmesh_2 (Variables|Default|GetStaticMesh))
  (bind _staticmesh_3 (Variables|Default|GetStaticMesh))
  (bind _returnvalue_2 (Transformation|GetWorldLocation _staticmesh))
  (bind _returnvalue_3 (Transformation|GetWorldRotation _staticmesh))
  (bind _asfirst_person_character (Utilities|Casting|CastToFirstPersonCharacter (Game|GetPlayerCharacter 0)))
  (bind (_out_hit _return_value) (Default|Trace _asfirst_person_character "TraceTypeQuery3"))
  (if _return_value
    (bind _asbp_board (Utilities|Casting|CastToBP_Board (.HitActor (Collision|BreakHitResult _out_hit)))
      (:then
        (if (== (Variables|/Game/Blueprints/PickUpObjects/BP_Board.BP_Board_C|GetCube _asbp_board) (.HitComponent (Collision|BreakHitResult _out_hit)))
          (if (not (Variables|/Game/Blueprints/PickUpObjects/BP_Interactable.BP_Interactable_C|GetCanPickUp? _asbp_board))
            (Input|DisableInput _asfirst_person_character _returnvalue)
            (Transformation|SetWorldLocationAndRotation _skeletalmesh_2 (Transformation|GetWorldLocation (Variables|/Game/Blueprints/PickUpObjects/BP_Board.BP_Board_C|GetSkeletalMesh _asbp_board)) (Transformation|GetWorldRotation (Variables|/Game/Blueprints/PickUpObjects/BP_Board.BP_Board_C|GetSkeletalMesh _asbp_board)) false true)
            (Rendering|SetVisibility _staticmesh_3 false false)
            (Rendering|SetVisibility _skeletalmesh_2 true false)
            (Components|Animation|PlayAnimation _skeletalmesh_2 "/Game/Objects/Meshes/Animated/nailpuller/hammer.hammer" false)
            (Utilities|FlowControl|Delay 1.46)
            (Physics|SetSimulatePhysics (Variables|/Game/Blueprints/PickUpObjects/BP_Interactable.BP_Interactable_C|GetStaticMesh _asbp_board) true)
            (Variables|/Game/Blueprints/PickUpObjects/BP_Interactable.BP_Interactable_C|SetCanPickUp? _asbp_board true)
            (Utilities|FlowControl|Delay 0.29)
            (Rendering|SetVisibility _staticmesh_3 true false)
            (Rendering|SetVisibility _skeletalmesh_2 false false)
            (Transformation|SetWorldLocationAndRotation _skeletalmesh_2 _returnvalue_2 _returnvalue_3 false true)
            (Input|EnableInput _asfirst_person_character _returnvalue))))
      (:CastFailed
        (bind _asbp_board_1 (Utilities|Casting|CastToBP_Board1 (.HitActor (Collision|BreakHitResult _out_hit))))
        (if (== (Variables|/Game/Blueprints/PickUpObjects/BP_Board1.BP_Board1_C|GetCube _asbp_board_1) (.HitComponent (Collision|BreakHitResult _out_hit)))
          (Input|DisableInput _asfirst_person_character _returnvalue)
          (Transformation|SetWorldLocationAndRotation _skeletalmesh (Transformation|GetWorldLocation (Variables|/Game/Blueprints/PickUpObjects/BP_Board1.BP_Board1_C|GetSkeletalMesh _asbp_board_1)) (Transformation|GetWorldRotation (Variables|/Game/Blueprints/PickUpObjects/BP_Board1.BP_Board1_C|GetSkeletalMesh _asbp_board_1)) false true)
          (Rendering|SetVisibility _staticmesh_2 false false)
          (Rendering|SetVisibility _skeletalmesh true false)
          (Components|Animation|PlayAnimation _skeletalmesh "/Game/Objects/Meshes/Animated/nailpuller/hammer.hammer" false)
          (Utilities|FlowControl|Delay 1.46)
          (Default|Break _asbp_board_1)
          (Utilities|FlowControl|Delay 0.29)
          (Rendering|SetVisibility _staticmesh_2 true false)
          (Rendering|SetVisibility _skeletalmesh false false)
          (Transformation|SetWorldLocationAndRotation _skeletalmesh _returnvalue_2 _returnvalue_3 false true)
          (Input|EnableInput _asfirst_person_character _returnvalue))))))

(fn ConstructionScript
  (|CallParentFunction))