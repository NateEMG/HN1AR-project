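; BP_Rifle is a rifle pickup that, when used, fires an explosion-style shot that flags DeadMan AI as shot.
; SetSocket takes the first-person character's Rifle as its socket.
; Use spawns an explosion emitter and sound, then finds every BP_DeadManAI overlapping Box1.
; Hits come from that box overlap rather than a trace, and each sets the IsShot blackboard key for the AI to handle.
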(event EventBeginPlay
  (|CallParentFunction) ; This node is disabled and will not be called.\nDrag off pins to build functionality.
)

(event Collision|EventActorBeginOverlap
  (params (OtherActor :type Actor%20Object%20Reference)))

(event EventTick
  (params (DeltaSeconds :type Float%20%28single-precision%29)))

(event EventSetSocket
  (bind _asfirst_person_character (Utilities|Casting|CastToFirstPersonCharacter (Game|GetPlayerCharacter 0)))
  (Variables|Default|SetSocket (Variables|/Game/Blueprints/Characters/FirstPersonBP/Blueprints/FirstPersonCharacter.FirstPersonCharacter_C|GetRifle _asfirst_person_character)))

(event EventUse
  (Effects|SpawnEmitteratLocation "/Game/StarterContent/Particles/P_Explosion.P_Explosion" (Transformation|GetWorldLocation (Variables|Default|GetScene)))
  (Audio|PlaySoundatLocation "/Game/StarterContent/Audio/Explosion_Cue.Explosion_Cue" (Transformation|GetActorLocation) "0, 0, 0" 1.0 1.0 0.0 "/Game/Sounds/Attenuation/DoorSoundAttenuation.DoorSoundAttenuation" 0 0)
  (for _array_element (Collision|GetOverlappingActors (Variables|Default|GetBox1) "/Game/NeighborInvasion/DeadManAI/BP_DeadManAI.BP_DeadManAI_C" :!class /Script/Engine.PrimitiveComponent)
    (AI|Components|Blackboard|SetValueasBool (AI|GetBlackboard _array_element) (Utilities|Name|MakeLiteralName "IsShot") true)))

(fn ConstructionScript
  (|CallParentFunction))