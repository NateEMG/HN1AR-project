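; Door actor that plays a cutscene when used, or a locked sound if locked, and handles AI passage.
; A placed chair locks it, disabling the smart nav link if it cannot be broken down.
; The link drives timed AI animations and door moves to open and reclose it, fail, or break the barricade.
; With two or more players, Tick re-applies the door transform after a delay when open or locked.
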(event OnSmartLinkReached(NavLink)
  (params (MovingActor :type Actor%20Object%20Reference) (DestinationPoint :type Vector%20%28by%20ref%29 :default "0, 0, 0"))
  (bind _door (Variables|Default|GetDoor))
  (Development|PrintString "open door")
  (bind _asai (Utilities|Casting|CastToAI MovingActor))
  (if (Variables|Default|GetCanAIOpen?)
    (if (Variables|Default|GetLocked)
      (if (Variables|Default|GetIsLockedWithChair?)
        (Audio|PlaySoundatLocation "/Game/Sounds/LockedDoor.LockedDoor" (Transformation|GetWorldLocation (Variables|Default|GetDoor)) "0, 0, 0" 1.0 1.0 0.0 "/Game/Sounds/Attenuation/DoorSoundAttenuation.DoorSoundAttenuation" 0 0)
        (Pawn|Components|CharacterMovement|DisableMovement (Variables|/Script/Engine.Character|GetCharacterMovement _asai))
        (if (Utilities|Enum|Equal(Enum) (Variables|/Game/Blueprints/Characters/AI2/AI.AI_C|GetCurrentState _asai) "NewEnumerator0")
          (if (Variables|Default|GetCanBreakDownDoorIdle?)
            (if (Variables|Default|GetCanBreakDownDoor?) :!label _label
              (Components|Animation|SetAnimationMode (Variables|/Script/Engine.Character|GetMesh _asai) "AnimationSingleNode")
              (Components|Animation|PlayAnimation (Variables|/Script/Engine.Character|GetMesh _asai) "/Game/Neighbor/Montages/pushdoor.pushdoor" false)
              (Utilities|FlowControl|Delay 4.2)
              (Variables|Default|SetIsLockedWithChair? false)
              (Variables|Default|SetLocked false)
              (Variables|Default|SetOpen true)
              (Physics|SetSimulatePhysics (Variables|/Game/Blueprints/PickUpObjects/BP_Interactable.BP_Interactable_C|GetStaticMesh (Variables|Default|GetSelectChair)) true)
              (Components|MoveComponentTo (Variables|Default|GetDoor) (Variables|Default|GetDoorOpen_Location) (Variables|Default|GetDoorOpen_Rotation) false false 0.1 false)
              (Utilities|FlowControl|Delay 0.2)
              (Components|Animation|SetAnimationMode (Variables|/Script/Engine.Character|GetMesh _asai) "AnimationBlueprint")
              (Pawn|Components|CharacterMovement|SetMovementMode (Variables|/Script/Engine.Character|GetCharacterMovement _asai) "MOVE_Walking" 0)
              (if (Utilities|Enum|Equal(Enum) (Variables|/Game/Blueprints/Characters/AI2/AI.AI_C|GetCurrentState _asai) "NewEnumerator0")
                (Class|BlackboardComponent|SetValueasInt (AI|GetBlackboard _asai) (Utilities|Name|MakeLiteralName "HuntTask") 1)
                (Default|SetState _asai "NewEnumerator2")
                (else
                  (Utilities|FlowControl|Delay 1.5 :!label _label_2)
                  (Components|MoveComponentTo _door (Variables|Default|GetDoorClose_Location) (Variables|Default|GetDoorClose_Rotation) false false (Variables|Default|GetOverTime) false)
                  (Audio|PlaySoundatLocation (Variables|Default|GetCloseSound) (Transformation|GetActorLocation) "0, 0, 0" 1.0 1.0 0.0 "/Game/Sounds/Attenuation/DoorSoundAttenuation.DoorSoundAttenuation" 0 0)
                  (Collision|SetCollisionEnabled (Variables|Default|GetDoor) "QueryAndPhysics")
                  (Variables|Default|SetOpen false)
                  (Variables|/Game/Blueprints/Characters/AI2/AI.AI_C|SetCanAIKick _asai true)))
              (else
                (bind _anim_length (Default|PlayAnimAI _asai "/Game/Neighbor/Animations/neighbour_lowpoly_Anim_rig_open_door_outward.neighbour_lowpoly_Anim_rig_open_door_outward" false :!label _label_3))
                (Utilities|FlowControl|Delay _anim_length)
                (Components|Animation|SetAnimationMode (Variables|/Script/Engine.Character|GetMesh _asai) "AnimationBlueprint")
                (Pawn|Components|CharacterMovement|SetMovementMode (Variables|/Script/Engine.Character|GetCharacterMovement _asai) "MOVE_Walking" 0)))
            (else
              (goto _label_3)))
          (else
            (goto _label)))
        (else
          (goto _label_3)))
      (elif (Variables|Default|GetOpen)
        (goto _label_2)
        (else
          (Variables|/Game/Blueprints/Characters/AI2/AI.AI_C|SetCanAIKick _asai false)
          (Pawn|Components|CharacterMovement|DisableMovement (Variables|/Script/Engine.Character|GetCharacterMovement _asai))
          (Components|Animation|SetAnimationMode (Variables|/Script/Engine.Character|GetMesh _asai) "AnimationSingleNode")
          (Components|Animation|PlayAnimation (Variables|/Script/Engine.Character|GetMesh _asai) "/Game/Neighbor/Animations/neighbour_lowpoly_Anim_rig_open_door_inward.neighbour_lowpoly_Anim_rig_open_door_inward" false)
          (Utilities|FlowControl|Delay 0.4)
          (Variables|Default|SetOpen true)
          (Audio|SpawnSoundatLocation (Variables|Default|GetOpenSound) (Transformation|GetActorLocation) "0, 0, 0" 1.0 1.0 0.0 "/Game/Sounds/Attenuation/DoorSoundAttenuation.DoorSoundAttenuation" 0)
          (Collision|SetCollisionEnabled (Variables|Default|GetDoor) "NoCollision")
          (Components|MoveComponentTo _door (Variables|Default|GetDoorOpen_Location) (Variables|Default|GetDoorOpen_Rotation) false false (Variables|Default|GetOverTime) false)
          (Utilities|FlowControl|Delay 0.54)
          (Components|Animation|SetAnimationMode (Variables|/Script/Engine.Character|GetMesh _asai) "AnimationBlueprint")
          (Pawn|Components|CharacterMovement|SetMovementMode (Variables|/Script/Engine.Character|GetCharacterMovement _asai) "MOVE_Walking" 0)
          (goto _label_2))))
    (elif (Utilities|Enum|Equal(Enum) (Variables|/Game/Blueprints/Characters/AI2/AI.AI_C|GetCurrentState _asai) "NewEnumerator0")
      (Default|RandomTask _asai))))

(event Custom|OpenClose
  (params (Component :type Primitive%20Component%20Object%20Reference))
  (if (== Component (Variables|Default|GetDoor))
    (if (Variables|Default|GetLocked)
      (Audio|PlaySoundatLocation "/Game/Sounds/LockedDoor_Cue.LockedDoor_Cue" (Transformation|GetWorldLocation (Variables|Default|GetScene)) "0, 0, 0" 1.0 1.0 0.0 "/Game/Sounds/Attenuation/DoorSoundAttenuation.DoorSoundAttenuation" 0 0)
      (else
        (bind _returnvalue (Sequencer|Player|CreateLevelSequencePlayer (Variables|Default|GetCutscene)))
        (Sequencer|Player|Play _returnvalue :!class /Script/MovieScene.MovieSceneSequencePlayer)
        (CallFunction|CutsceneTriggered)))))

(event Custom|CheckIfOpenOnServer
  (Utilities|FlowControl|Sequence
    (:then_0
      (if (Variables|Default|GetOpen)
        (CallFunction|OpenClientDoors :!label _label)))
    (:then_1
      (if (Variables|Default|GetLocked)
        (goto _label)))))

(event Custom|OpenClient)

(event Custom|OpenClientDoors
  (bind _door (Variables|Default|GetDoor))
  (if (Variables|Default|GetOpen)
    (Transformation|SetRelativeLocationAndRotation _door (Variables|Default|GetDoorOpen_Location) (Variables|Default|GetDoorOpen_Rotation) false false)
    (else
      (Transformation|SetRelativeLocationAndRotation _door (Variables|Default|GetDoorClose_Location) (Variables|Default|GetDoorClose_Rotation) false false))))

(event Custom|OnSmartLinkReached_Event_0
  (params (MovingActor :type Actor%20Object%20Reference) (DestinationPoint :type Vector%20%28by%20ref%29)))

(event Custom|SetChair
  (params (SelectChair :type BP%20Chair%20Object%20Reference))
  (bind _stool (Variables|Default|GetStool))
  (bind _output_get (Variables|Default|SetSelectChair SelectChair))
  (Transformation|SetActorLocationAndRotation _output_get (Transformation|GetWorldLocation _stool) (Transformation|GetWorldRotation _stool) false true)
  (Physics|SetSimulatePhysics (Variables|/Game/Blueprints/PickUpObjects/BP_Interactable.BP_Interactable_C|GetStaticMesh _output_get) false)
  (Variables|Default|SetLocked true)
  (Variables|Default|SetIsLockedWithChair? true)
  (if (not (Variables|Default|GetCanBreakDownDoor?))
    (Class|NavLinkProxy|SetSmartLinkEnabled (Variables|Default|GetNavLink) false)))

(event Custom|CutsceneTriggered)

(event EventBeginPlay
  (bind _door (Variables|Default|GetDoor))
  (Utilities|FlowControl|Sequence
    (:then_0
      (if (Variables|Default|GetOpen)
        (Transformation|SetRelativeLocationAndRotation _door (Variables|Default|GetDoorOpen_Location) (Variables|Default|GetDoorOpen_Rotation) false false)
        (Variables|Default|SetOpen true)
        (else
          (Transformation|SetRelativeLocationAndRotation _door (Variables|Default|GetDoorClose_Location) (Variables|Default|GetDoorClose_Rotation) false false)
          (Variables|Default|SetOpen false))))))

(event EventTick
  (params (DeltaSeconds :type Float%20%28single-precision%29))
  (Utilities|FlowControl|Sequence
    (:then_0
      (bind _asgame_instance_hnar (Utilities|Casting|CastToGameInstanceHNAR (Game|GetGameInstance)))
      (if (>= (Class|FindSessionsCallbackProxy|GetCurrentPlayers (Variables|/Game/GameInstanceHNAR.GameInstanceHNAR_C|GetSession _asgame_instance_hnar)) 2)
        (Utilities|FlowControl|Delay 1.0)
        (CallFunction|CheckifOpenonServer)))))

(fn ConstructionScript)