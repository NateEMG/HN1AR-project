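; Breakable window with three destructible panes that alerts the AI when smashed and becomes a route it can pass through.
; Each pane's first fracture plays glass audio and, if the AI can hear, reports noise, stores an investigate transform, enables that pane's initially disabled smart link and writes the window to the blackboard.
; Reaching a link turns the AI toward the window and briefly disables capsule and mesh collision.
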(event OnComponentFracture(Destructible)
  (params (HitPoint :type Vector%20%28by%20ref%29 :default "0, 0, 0") (HitDirection :type Vector%20%28by%20ref%29 :default "0, 0, 0"))
  (bind _self self)
  (bind _smartlink1 (Variables|Default|GetSmartLink1))
  (bind _arrow (Variables|Default|GetArrow))
  (Utilities|FlowControl|DoOnce false
    (:Completed
      (Audio|PlaySoundatLocation "/Game/Sounds/GlassBreak.GlassBreak" (Transformation|GetActorLocation (Components|GetOwner (Variables|Default|GetDestructible))) "0, 0, 0" 1.0 1.0 0.0 "/Game/Sounds/Attenuation/DoorSoundAttenuation.DoorSoundAttenuation" 0 0)
      (if (Variables|/Game/Blueprints/Characters/AI2/AI.AI_C|GetCanHear (Variables|Default|GetAI))
        (Class|AISenseHearing|ReportNoiseEvent (Transformation|GetWorldLocation _arrow) 5.0 _self 6e+02 "Window")
        (Variables|Default|SetInvestigateTransform (Transformation|GetWorldTransform _arrow))
        (Utilities|FlowControl|Sequence
          (:then_0
            (Utilities|IsValid _smartlink1
              (:Is%20Valid
                (Class|NavLinkProxy|SetSmartLinkEnabled _smartlink1 true))))
          (:then_1
            (AI|Components|Blackboard|SetValueasObject (AI|GetBlackboard (Variables|Default|GetAI)) (Utilities|Name|MakeLiteralName "ObjectRef") _self)))))))

(event OnComponentFracture(Destructible1)
  (params (HitPoint :type Vector%20%28by%20ref%29 :default "0, 0, 0") (HitDirection :type Vector%20%28by%20ref%29 :default "0, 0, 0"))
  (bind _self self)
  (bind _smartlink2 (Variables|Default|GetSmartLink2))
  (bind _arrow1 (Variables|Default|GetArrow1))
  (Utilities|FlowControl|DoOnce false
    (:Completed
      (Audio|PlaySoundatLocation "/Game/Sounds/GlassBreak.GlassBreak" (Transformation|GetActorLocation (Components|GetOwner (Variables|Default|GetDestructible1))) "0, 0, 0" 1.0 1.0 0.0 "/Game/Sounds/Attenuation/DoorSoundAttenuation.DoorSoundAttenuation" 0 0)
      (if (Variables|/Game/Blueprints/Characters/AI2/AI.AI_C|GetCanHear (Variables|Default|GetAI))
        (Class|AISenseHearing|ReportNoiseEvent (Transformation|GetWorldLocation _arrow1) 5.0 _self 6e+02 "Window")
        (Variables|Default|SetInvestigateTransform (Transformation|GetWorldTransform _arrow1))
        (Utilities|FlowControl|Sequence
          (:then_0
            (Utilities|IsValid _smartlink2
              (:Is%20Valid
                (Class|NavLinkProxy|SetSmartLinkEnabled _smartlink2 true))))
          (:then_1
            (AI|Components|Blackboard|SetValueasObject (AI|GetBlackboard (Variables|Default|GetAI)) (Utilities|Name|MakeLiteralName "ObjectRef") _self)))))))

(event OnComponentFracture(Destructible2)
  (params (HitPoint :type Vector%20%28by%20ref%29 :default "0, 0, 0") (HitDirection :type Vector%20%28by%20ref%29 :default "0, 0, 0"))
  (bind _self self)
  (bind _smartlink3 (Variables|Default|GetSmartLink3))
  (bind _arrow2 (Variables|Default|GetArrow2))
  (Utilities|FlowControl|DoOnce false
    (:Completed
      (Audio|PlaySoundatLocation "/Game/Sounds/GlassBreak.GlassBreak" (Transformation|GetActorLocation (Components|GetOwner (Variables|Default|GetDestructible2))) "0, 0, 0" 1.0 1.0 0.0 "/Game/Sounds/Attenuation/DoorSoundAttenuation.DoorSoundAttenuation" 0 0)
      (if (Variables|/Game/Blueprints/Characters/AI2/AI.AI_C|GetCanHear (Variables|Default|GetAI))
        (Class|AISenseHearing|ReportNoiseEvent (Transformation|GetWorldLocation _arrow2) 5.0 _self 6e+02 "Window")
        (Variables|Default|SetInvestigateTransform (Transformation|GetWorldTransform _arrow2))
        (Utilities|FlowControl|Sequence
          (:then_0
            (Utilities|IsValid _smartlink3
              (:Is%20Valid
                (Class|NavLinkProxy|SetSmartLinkEnabled _smartlink3 true))))
          (:then_1
            (AI|Components|Blackboard|SetValueasObject (AI|GetBlackboard (Variables|Default|GetAI)) (Utilities|Name|MakeLiteralName "ObjectRef") _self)))))))

(event OnSmartLinkReached(SmartLink2)
  (params (MovingActor :type Actor%20Object%20Reference) (DestinationPoint :type Vector%20%28by%20ref%29 :default "0, 0, 0"))
  (bind _ai (Variables|Default|GetAI))
  (bind _capsulecomponent (Variables|/Script/Engine.Character|GetCapsuleComponent _ai))
  (Transformation|SetActorRotation _ai (Math|Rotator|MakeRotator 0.0 0.0 (.yaw (Math|Rotator|FindLookatRotation (Transformation|GetActorLocation _ai) (Transformation|GetActorLocation)))))
  (Collision|SetCollisionEnabled _capsulecomponent "NoCollision")
  (Utilities|FlowControl|Delay 0.7)
  (Collision|SetCollisionEnabled _capsulecomponent "QueryAndPhysics")
  (Utilities|FlowControl|RetriggerableDelay 0.5)
  (Collision|SetCollisionEnabled (Variables|Default|GetStaticMesh1) "QueryAndPhysics"))

(event OnSmartLinkReached(SmartLink1)
  (params (MovingActor :type Actor%20Object%20Reference) (DestinationPoint :type Vector%20%28by%20ref%29 :default "0, 0, 0"))
  (bind _ai (Variables|Default|GetAI))
  (bind _capsulecomponent (Variables|/Script/Engine.Character|GetCapsuleComponent _ai))
  (Transformation|SetActorRotation _ai (Math|Rotator|MakeRotator 0.0 0.0 (.yaw (Math|Rotator|FindLookatRotation (Transformation|GetActorLocation _ai) (Transformation|GetActorLocation)))))
  (Collision|SetCollisionEnabled _capsulecomponent "NoCollision")
  (Utilities|FlowControl|Delay 0.7)
  (Collision|SetCollisionEnabled _capsulecomponent "QueryAndPhysics")
  (Utilities|FlowControl|RetriggerableDelay 0.5)
  (Collision|SetCollisionEnabled (Variables|Default|GetStaticMesh1) "QueryAndPhysics"))

(event OnSmartLinkReached(SmartLink3)
  (params (MovingActor :type Actor%20Object%20Reference) (DestinationPoint :type Vector%20%28by%20ref%29 :default "0, 0, 0"))
  (bind _ai (Variables|Default|GetAI))
  (bind _capsulecomponent (Variables|/Script/Engine.Character|GetCapsuleComponent _ai))
  (Transformation|SetActorRotation _ai (Math|Rotator|MakeRotator 0.0 0.0 (.yaw (Math|Rotator|FindLookatRotation (Transformation|GetActorLocation _ai) (Transformation|GetActorLocation)))))
  (Collision|SetCollisionEnabled _capsulecomponent "NoCollision")
  (Utilities|FlowControl|Delay 0.7)
  (Collision|SetCollisionEnabled _capsulecomponent "QueryAndPhysics")
  (Utilities|FlowControl|RetriggerableDelay 0.5)
  (Collision|SetCollisionEnabled (Variables|Default|GetStaticMesh1) "QueryAndPhysics"))

(event EventBeginPlay
  (bind _smartlink2 (Variables|Default|GetSmartLink2))
  (bind _smartlink3 (Variables|Default|GetSmartLink3))
  (bind _smartlink1 (Variables|Default|GetSmartLink1))
  (bind _returnvalue (Actor|GetActorOfClass "/Game/Blueprints/Characters/AI2/AI.AI_C"))
  (Variables|Default|SetAI _returnvalue)
  (Utilities|FlowControl|Sequence
    (:then_0
      (Utilities|IsValid _smartlink1
        (:Is%20Valid
          (Class|NavLinkProxy|SetSmartLinkEnabled _smartlink1 false))))
    (:then_1
      (Utilities|IsValid _smartlink2
        (:Is%20Valid
          (Class|NavLinkProxy|SetSmartLinkEnabled _smartlink2 false))))
    (:then_2
      (Utilities|IsValid _smartlink3
        (:Is%20Valid
          (Class|NavLinkProxy|SetSmartLinkEnabled _smartlink3 false))))))

(fn ConstructionScript)