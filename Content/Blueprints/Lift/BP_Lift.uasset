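; BP_Lift is a powered elevator with four floor buttons that carries its cabin mesh between referenced floor actors.
; PressedButton sets the target floor and calls MoveElevator, with DoOnce gates blocking further requests until the trip ends.
; MoveElevator closes cabin and landing doors, moves with audio over a time scaled by floor distance, then reopens both.
; Later Sequence pins compute that distance and cache the target during the door-closing delay.
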(event Custom|PressedButton
  (params (Component :type Primitive%20Component%20Object%20Reference))
  (if (Variables|Default|GetPowered?)
    (if (== Component (Variables|Default|Getbutton1))
      (Variables|Default|SetFloorPressed 0)
      (Utilities|FlowControl|DoOnce false :!label _label
        (:Completed
          (CallFunction|MoveElevator)
          (Audio|PlaySoundatLocation "/Game/Sounds/train_room_button.train_room_button" (Transformation|GetWorldLocation Component) "0, 0, 0" 1.0 1.0 0.0 "/Game/Sounds/Attenuation/ItemAtten.ItemAtten" 0 0)))
      (elif (== Component (Variables|Default|Getbutton2))
        (Variables|Default|SetFloorPressed 1)
        (goto _label)
        (elif (== Component (Variables|Default|Getbutton3))
          (Variables|Default|SetFloorPressed 2)
          (goto _label)
          (elif (== Component (Variables|Default|Getbutton4))
            (Variables|Default|SetFloorPressed 3)
            (goto _label)))))))

(event Custom|MoveElevator
  (bind _audio (Variables|Default|GetAudio))
  (if (Variables|Default|GetPowered?)
    (if (== (Variables|Default|GetFloorPressed) (Variables|Default|GetCurrentFloor))
      (Utilities|FlowControl|DoOnce false) ; enters at Reset
      (else
        (Utilities|FlowControl|DoOnce false :!label _label
          (:Completed
            (Utilities|FlowControl|Sequence
              (:then_0
                (Default|Close (Utilities|Array|Get(acopy) (Variables|Default|GetLiftDoors) (Variables|Default|GetCurrentFloor)))
                (CallFunction|CloseDoors)
                (Utilities|FlowControl|Delay 1.0)
                (Audio|Components|Audio|Play _audio 0.0)
                (Components|MoveComponentTo (Variables|Default|GetStaticMesh) (Transformation|GetActorLocation (Utilities|Array|Get(acopy) (Variables|Default|GetFloors) (Variables|Default|GetFloorPressed))) "0, 0, 0" false false (* (Variables|Default|GetDistance) (Variables|Default|GetLiftTime)) false)
                (Audio|Components|Audio|Stop _audio)
                (bind _output_get (Variables|Default|SetCurrentFloor (Variables|Default|GetFloorPressedTEMP)))
                (Variables|Default|SetFloorPressed -1)
                (Default|Open (Utilities|Array|Get(acopy) (Variables|Default|GetLiftDoors) _output_get))
                (CallFunction|OpenDoors)
                (Utilities|FlowControl|Delay 1.5)
                (Utilities|FlowControl|Sequence
                  (:then_0
                    (Utilities|FlowControl|DoOnce false) ; enters at Reset
                  )
                  (:then_1
                    (goto _label Reset))))
              (:then_1
                (if (> (- (Variables|Default|GetFloorPressed) (Variables|Default|GetCurrentFloor)) (Variables|Default|GetCurrentFloor))
                  (bind _output_get_2 (Variables|Default|SetDistance (- (Variables|Default|GetFloorPressed) (Variables|Default|GetCurrentFloor)) :!label _label_2))
                  (Development|PrintString (Utilities|String|ToString(Integer) _output_get_2))
                  (elif (== (- (Variables|Default|GetFloorPressed) (Variables|Default|GetCurrentFloor)) 1)
                    (goto _label_2)
                    (else
                      (bind _output_get_3 (Variables|Default|SetDistance (* (- (Variables|Default|GetFloorPressed) (Variables|Default|GetCurrentFloor)) -1)))
                      (Development|PrintString (Utilities|String|ToString(Integer) _output_get_3))))))
              (:then_2
                (Variables|Default|SetFloorPressedTEMP (Variables|Default|GetFloorPressed))))))))))

(event Custom|OpenDoors
  (Utilities|FlowControl|Sequence
    (:then_0
      (Components|MoveComponentTo (Variables|Default|Getdoor) "75.000000,106.000000,-3.000000" "0, 0, 0" false false 1.0 false))
    (:then_1
      (Components|MoveComponentTo (Variables|Default|Getdoor1) "-75.000000,106.000000,-3.000000" "0, 0, 0" false false 1.0 false))))

(event Custom|CloseDoors
  (Utilities|FlowControl|Sequence
    (:then_0
      (Components|MoveComponentTo (Variables|Default|Getdoor) "25.000000,106.000000,-3.000000" "0, 0, 0" false false 1.0 false))
    (:then_1
      (Components|MoveComponentTo (Variables|Default|Getdoor1) "-25.000000,106.000000,-3.000000" "0, 0, 0" false false 1.0 false))))

(event EventBeginPlay)

(event Collision|EventActorBeginOverlap
  (params (OtherActor :type Actor%20Object%20Reference)))

(event EventTick
  (params (DeltaSeconds :type Float%20%28single-precision%29)))

(fn ConstructionScript)