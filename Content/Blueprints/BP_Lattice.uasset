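; BP_Lattice is a metal gate whose mesh slides up and down through its Open and Close events, with a sound for each.
; An optional PowerSwitch gates movement: an unpowered switch blocks sound and motion, though IsOpen still updates, while no switch lets the gate move freely.
; Two latent MoveComponentTo nodes drive opposite directions, each event starting one and stopping the other so movement can reverse midway.
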(event Custom|Open
  (bind _staticmesh (Variables|Default|GetStaticMesh))
  (bind _powerswitch (Variables|Default|GetPowerSwitch))
  (Variables|Default|SetIsOpen true)
  (Utilities|IsValid _powerswitch
    (:Is%20Valid
      (if (Variables|/Game/Blueprints/BP_PowerSwitch.BP_PowerSwitch_C|GetPowerWorking? _powerswitch)
        (Audio|PlaySoundatLocation "/Game/Sounds/gate_open_metal_1.gate_open_metal_1" (Transformation|GetActorLocation) "0, 0, 0" 1.0 1.0 0.0 "/Game/Sounds/Attenuation/NeighborVoiceAtten.NeighborVoiceAtten" 0 0 :!label _label)
        (Utilities|FlowControl|Sequence
          (:then_0
            (Components|MoveComponentTo _staticmesh "0, 0,335.000000" "0, 0, 0" false false 2.5 false))
          (:then_1
            (Components|MoveComponentTo _staticmesh "0, 0, 0" "0, 0, 0" false false 2.5 false) ; enters at Stop
          ))))
    (:Is%20Not%20Valid
      (goto _label))))

(event Custom|Close
  (bind _staticmesh (Variables|Default|GetStaticMesh))
  (bind _powerswitch (Variables|Default|GetPowerSwitch))
  (Variables|Default|SetIsOpen false)
  (Utilities|IsValid _powerswitch
    (:Is%20Valid
      (if (Variables|/Game/Blueprints/BP_PowerSwitch.BP_PowerSwitch_C|GetPowerWorking? _powerswitch)
        (Audio|PlaySoundatLocation "/Game/Sounds/gate_close_metal_2.gate_close_metal_2" (Transformation|GetActorLocation) "0, 0, 0" 1.0 1.0 0.0 "/Game/Sounds/Attenuation/DoorSoundAttenuation.DoorSoundAttenuation" 0 0 :!label _label)
        (Utilities|FlowControl|Sequence
          (:then_0
            (Components|MoveComponentTo _staticmesh "0, 0, 0" "0, 0, 0" false false 2.5 false))
          (:then_1
            (Components|MoveComponentTo _staticmesh "0, 0,335.000000" "0, 0, 0" false false 2.5 false) ; enters at Stop
          ))))
    (:Is%20Not%20Valid
      (goto _label))))

(fn ConstructionScript)