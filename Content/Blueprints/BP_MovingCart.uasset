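; Cart hazard that rides a referenced track's spline and sends the player back to spawn on contact.
; A Mover timeline, rate-scaled by Duration and begun at StartOffset, sets location and rotation along the spline, replaying from the start after random pauses.
; The first run waits a random delay, plus a long hold if HasPlayed is false.
; Box2 overlap plays a fade and death sound, then restores the player's spawn location and view rotation.
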(event OnComponentBeginOverlap(Box2)
  (params (OverlappedComponent :type Primitive%20Component%20Object%20Reference) (OtherActor :type Actor%20Object%20Reference) (OtherComp :type Primitive%20Component%20Object%20Reference) (OtherBodyIndex :type Integer) (bFromSweep :type Boolean) (SweepResult :type Hit%20Result%20Structure%20%28by%20ref%29))
  (bind _asfirst_person_character (Utilities|Casting|CastToFirstPersonCharacter OtherActor))
  (UserInterface|Animation|PlayAnimation (Variables|/Game/Blueprints/Characters/FirstPersonBP/Blueprints/FirstPersonCharacter.FirstPersonCharacter_C|GetFadeAnim _asfirst_person_character) (Variables|/Game/Blueprints/Characters/AI2/FadeAnimation.FadeAnimation_C|Getfadein (Variables|/Game/Blueprints/Characters/FirstPersonBP/Blueprints/FirstPersonCharacter.FirstPersonCharacter_C|GetFadeAnim _asfirst_person_character)) 0.0 1 "Forward" 1.0 false)
  (Audio|PlaySound2D "/Game/Sounds/hit/fall_dead_2_Cue.fall_dead_2_Cue" 1.0 1.0 0.0 0 0)
  (Transformation|SetActorLocation _asfirst_person_character (.location (Variables|/Game/Blueprints/Characters/FirstPersonBP/Blueprints/FirstPersonCharacter.FirstPersonCharacter_C|GetSpawnTransform _asfirst_person_character)) false false)
  (Pawn|SetControlRotation (Game|GetPlayerController 0) (.rotation (Variables|/Game/Blueprints/Characters/FirstPersonBP/Blueprints/FirstPersonCharacter.FirstPersonCharacter_C|GetSpawnTransform _asfirst_person_character))))

(event Custom|MoveCart
  (bind _mover (Variables|Default|GetMover))
  (bind _trackref (Variables|Default|GetTrackRef))
  (bind _spline (Variables|/Game/Blueprints/BP_Spline.BP_Spline_C|GetSpline _trackref))
  (Components|Timeline|SetPlayRate _mover (/ 1.0 (Variables|Default|GetDuration)))
  (Components|Timeline|SetNewTime _mover (Variables|Default|GetStartOffset))
  (bind _alpha (Timeline|Mover Play)
    (:Update
      (Variables|Default|SetAlpha _alpha)
      (Transformation|SetActorLocationAndRotation (Spline|GetLocationatDistanceAlongSpline _spline (Math|Float|Lerp 0.0 (Spline|GetSplineLength _spline) (Variables|Default|GetAlpha)) "World") (Spline|GetRotationatDistanceAlongSpline _spline (Math|Float|Lerp 0.0 (Spline|GetSplineLength _spline) (Variables|Default|GetAlpha)) "World")))
    (:Finished
      (Utilities|FlowControl|Delay (Math|Conversions|ToFloat(Integer) (Math|Random|RandomIntegerinRange 5 60)))
      (Timeline|Mover PlayFromStart))))

(event EventBeginPlay
  (Utilities|FlowControl|Delay 0.2)
  (bind _asfirst_person_character (Utilities|Casting|CastToFirstPersonCharacter (Game|GetPlayerCharacter 0)))
  (if (Variables|/Game/Blueprints/Characters/FirstPersonBP/Blueprints/FirstPersonCharacter.FirstPersonCharacter_C|GethasPlayed? _asfirst_person_character)
    _
    (else
      (Utilities|FlowControl|Delay 50.5)))
  (Utilities|FlowControl|Delay (Math|Conversions|ToFloat(Integer) (Math|Random|RandomIntegerinRange 5 60)))
  (CallFunction|MoveCart))

(fn ConstructionScript)