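; BP_LadderDoor_w_bolt is a bolted double ladder door that opens and records its unlock in the save data.
; Open, or OpenBolt given either bolt mesh, hides both bolts, disables their collision, moves and rotates the two door meshes apart, and plays a creak.
; It then sets the Alpha2 or Act 2 ladder flag based on the current level name and saves puzzle data through GameInstanceHNAR.
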(event Custom|OpenBolt
  (params (Component :type Actor%20Component%20Object%20Reference))
  (bind _staticmesh2 (Variables|Default|GetStaticMesh2))
  (if (== Component _staticmesh2)
    (Collision|SetCollisionEnabled _staticmesh2 "NoCollision" :!label _label)
    (Rendering|SetVisibility _staticmesh2 false false)
    (Utilities|FlowControl|Sequence
      (:then_0
        (Components|MoveComponentTo (Variables|Default|GetStaticMesh) "-58.000000, 0, 0" "0,90.000000, 0" false false 1.0 false))
      (:then_1
        (Components|MoveComponentTo (Variables|Default|GetStaticMesh1) "58.000000, 0, 0" "0,-90.000000, 0" false false 1.0 false))
      (:then_2
        (Audio|PlaySoundatLocation "/Game/Sounds/metallic_creak.metallic_creak" (Transformation|GetWorldLocation (Variables|Default|GetArrow)) "0, 0, 0" 1.0 1.0 0.0 "/Game/Sounds/Attenuation/DoorSoundAttenuation.DoorSoundAttenuation" 0 0))
      (:then_3
        (bind _asgame_instance_hnar (Utilities|Casting|CastToGameInstanceHNAR (Game|GetGameInstance)))
        (bind _returnvalue (Game|GetCurrentLevelName true))
        (if (Utilities|Enum|Equal(Enum) _returnvalue "Alpha2")
          (Variables|/Game/SaveData.SaveData_C|SetunlockedLadder (Variables|/Game/GameInstanceHNAR.GameInstanceHNAR_C|GetAs%20Save%20Data _asgame_instance_hnar) true)
          (else
            (Variables|/Game/SaveData.SaveData_C|SetunlockedLadderAct2 (Variables|/Game/GameInstanceHNAR.GameInstanceHNAR_C|GetAs%20Save%20Data _asgame_instance_hnar) true)))
        (Default|SavePuzzleData _asgame_instance_hnar)))
    (elif (== Component (Variables|Default|GetStaticMesh3))
      (goto _label))))

(event Custom|Open
  (bind _staticmesh2 (Variables|Default|GetStaticMesh2))
  (Collision|SetCollisionEnabled _staticmesh2 "NoCollision")
  (Rendering|SetVisibility _staticmesh2 false false)
  (Utilities|FlowControl|Sequence
    (:then_0
      (Components|MoveComponentTo (Variables|Default|GetStaticMesh) "-58.000000, 0, 0" "0,90.000000, 0" false false 1.0 false))
    (:then_1
      (Components|MoveComponentTo (Variables|Default|GetStaticMesh1) "58.000000, 0, 0" "0,-90.000000, 0" false false 1.0 false))
    (:then_2
      (Audio|PlaySoundatLocation "/Game/Sounds/metallic_creak.metallic_creak" (Transformation|GetWorldLocation (Variables|Default|GetArrow)) "0, 0, 0" 1.0 1.0 0.0 "/Game/Sounds/Attenuation/DoorSoundAttenuation.DoorSoundAttenuation" 0 0))
    (:then_3
      (bind _asgame_instance_hnar (Utilities|Casting|CastToGameInstanceHNAR (Game|GetGameInstance)))
      (bind _returnvalue (Game|GetCurrentLevelName true))
      (if (Utilities|Enum|Equal(Enum) _returnvalue "Alpha2")
        (Variables|/Game/SaveData.SaveData_C|SetunlockedLadder (Variables|/Game/GameInstanceHNAR.GameInstanceHNAR_C|GetAs%20Save%20Data _asgame_instance_hnar) true)
        (else
          (Variables|/Game/SaveData.SaveData_C|SetunlockedLadderAct2 (Variables|/Game/GameInstanceHNAR.GameInstanceHNAR_C|GetAs%20Save%20Data _asgame_instance_hnar) true)))
      (Default|SavePuzzleData _asgame_instance_hnar))))

(event EventBeginPlay)

(fn ConstructionScript)