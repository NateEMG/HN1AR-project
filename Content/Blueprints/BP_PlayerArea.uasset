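; BP_PlayerArea is a trigger box that makes the AI break off when it enters in a specific state while seeing the player.
; On overlap it freezes movement, disables chase and hearing, and plays the "it's a trap" animation for a timed delay.
; It then starts a random task, restores walking and hearing, and clears perception.
; Older player-side logic toggling neighbor chase, catch and perception remains unconnected.
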(event OnComponentBeginOverlap(Box)
  (params (OverlappedComponent :type Primitive%20Component%20Object%20Reference) (OtherActor :type Actor%20Object%20Reference) (OtherComp :type Primitive%20Component%20Object%20Reference) (OtherBodyIndex :type Integer) (bFromSweep :type Boolean) (SweepResult :type Hit%20Result%20Structure%20%28by%20ref%29))
  (bind _ai (Variables|Default|GetAI))
  (bind _charactermovement (Variables|/Script/Engine.Character|GetCharacterMovement _ai))
  (bind _asai (Utilities|Casting|CastToAI OtherActor))
  (if (and (Utilities|Enum|Equal(Enum) (Variables|/Game/Blueprints/Characters/AI2/AI.AI_C|GetCurrentState _ai) "NewEnumerator4") (Variables|/Game/Blueprints/Characters/AI2/AI.AI_C|GetCanSeePlayer _ai))
    (Pawn|Components|CharacterMovement|DisableMovement _charactermovement)
    (Default|SetState _ai "NewEnumerator7")
    (Variables|/Game/Blueprints/Characters/AI2/AI.AI_C|SetCanChase _ai false)
    (Variables|/Game/Blueprints/Characters/AI2/AI.AI_C|SetCanHear _ai false)
    (bind _anim_length (Default|PlayAnimAI _ai "/Game/Neighbor/Animations/neighbour_lowpoly_Anim_rig_it_s_a_trap_.neighbour_lowpoly_Anim_rig_it_s_a_trap_" true))
    (Utilities|FlowControl|Delay _anim_length)
    (Default|RandomTask _ai)
    (Default|SetState _ai "NewEnumerator0")
    (Pawn|Components|CharacterMovement|SetMovementMode _charactermovement "MOVE_Walking" 0)
    (Utilities|FlowControl|Delay 0.5)
    (Variables|/Game/Blueprints/Characters/AI2/AI.AI_C|SetCanSeePlayer _ai false)
    (Variables|/Game/Blueprints/Characters/AI2/AI.AI_C|SetCanHear _ai true)
    (Class|AIPerceptionComponent|ForgetAll (Variables|/Game/Blueprints/Characters/AI2/AI.AI_C|GetAIPerception _ai))))

(fn ConstructionScript)