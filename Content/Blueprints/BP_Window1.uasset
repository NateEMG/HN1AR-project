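; Breakable window that alerts the AI and becomes a path for it once shattered.
; On first fracture it plays a glass sound and, if the AI can hear, reports a noise, sets itself as the blackboard investigate object and enables its smart nav link.
; When the link is reached, it turns the AI toward the window and briefly disables capsule and mesh collision to let it pass.
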(event OnSmartLinkReached(NavLink)
  (params (MovingActor :type Actor%20Object%20Reference) (DestinationPoint :type Vector%20%28by%20ref%29 :default "0, 0, 0"))
  (bind _ai (Variables|Default|GetAI))
  (bind _capsulecomponent (Variables|/Script/Engine.Character|GetCapsuleComponent _ai))
  (Transformation|SetActorRotation _ai (Math|Rotator|MakeRotator 0.0 0.0 (.yaw (Math|Rotator|FindLookatRotation (Transformation|GetActorLocation _ai) (Transformation|GetActorLocation)))))
  (Collision|SetCollisionEnabled _capsulecomponent "NoCollision")
  (Utilities|FlowControl|Delay 0.7)
  (Collision|SetCollisionEnabled _capsulecomponent "QueryAndPhysics")
  (Utilities|FlowControl|RetriggerableDelay 0.5)
  (Collision|SetCollisionEnabled (Variables|Default|GetStaticMesh) "QueryAndPhysics"))

(event OnComponentFracture(Destructible)
  (params (HitPoint :type Vector%20%28by%20ref%29 :default "0, 0, 0") (HitDirection :type Vector%20%28by%20ref%29 :default "0, 0, 0"))
  (bind _self self)
  (bind _arrow (Variables|Default|GetArrow))
  (Utilities|FlowControl|DoOnce false
    (:Completed
      (Audio|PlaySoundatLocation "/Game/Sounds/GlassBreak.GlassBreak" (Transformation|GetActorLocation (Components|GetOwner (Variables|Default|GetDestructible))) "0, 0, 0" 1.0 1.0 0.0 "/Game/Sounds/Attenuation/DoorSoundAttenuation.DoorSoundAttenuation" 0 0)
      (if (Variables|/Game/Blueprints/Characters/AI2/AI.AI_C|GetCanHear (Variables|Default|GetAI))
        (Class|AISenseHearing|ReportNoiseEvent (Transformation|GetWorldLocation _arrow) 5.0 _self 6e+02 "Window")
        (Utilities|FlowControl|Sequence
          (:then_0
            (Variables|Default|SetInvestigateTransform (Transformation|GetWorldTransform _arrow))
            (AI|Components|Blackboard|SetValueasObject (AI|GetBlackboard (Variables|Default|GetAI)) (Utilities|Name|MakeLiteralName "ObjectRef") _self))
          (:then_1
            (Class|NavLinkProxy|SetSmartLinkEnabled (Variables|Default|GetNavLink) true)
            (Variables|Default|SetIsBroken true)))))))

(event OnComponentBeginOverlap(Box)
  (params (OverlappedComponent :type Primitive%20Component%20Object%20Reference) (OtherActor :type Actor%20Object%20Reference) (OtherComp :type Primitive%20Component%20Object%20Reference) (OtherBodyIndex :type Integer) (bFromSweep :type Boolean) (SweepResult :type Hit%20Result%20Structure%20%28by%20ref%29)))

(event EventBeginPlay
  (bind _navlink (Variables|Default|GetNavLink))
  (bind _returnvalue (Actor|GetActorOfClass "/Game/Blueprints/Characters/AI2/AI.AI_C"))
  (Variables|Default|SetAI _returnvalue)
  (Utilities|IsValid _navlink
    (:Is%20Valid
      (if (not (Variables|Default|GetIsBroken))
        (Class|NavLinkProxy|SetSmartLinkEnabled _navlink false)))))

(event EventTick
  (params (DeltaSeconds :type Float%20%28single-precision%29)))

(fn ConstructionScript)